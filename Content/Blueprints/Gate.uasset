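; Gate actor that unlocks and swings open when something overlaps its Collider, with no check on which actor it is.
; UnlockGate swaps the iron fence gate mesh to its unlocked version, activates the UnlockDoor component and destroys the Collider so the trigger fires only once.
; The Open timeline then drives the gate's relative yaw from its Progress track to swing it open.
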(event `UnlockGate`
  (`StaticMeshComponent.SetStaticMesh` (`self.Gate`) "/Game/Environment/meshes/fence/SM_fenceIron_gateSmall_unlocked.SM_fenceIron_gateSmall_unlocked")
  (`ActorComponent.Activate` (`self.UnlockDoor`) false)
  (`ActorComponent.K2_DestroyComponent` (`self.Collider`))
  (bind (_direction _progress) (`Timeline|Open`)
    (:`Update`
      (`SceneComponent.K2_SetRelativeRotation` (`self.Gate`) (`KismetMathLibrary.MakeRotator` 0.0 0.0 (* _progress -160.0)) false false))))

(event `self.Collider.OnComponentBeginOverlap`
  (params (OverlappedComponent :type "PrimitiveComponent Object Reference") (OtherActor :type "Actor Object Reference") (OtherComp :type "PrimitiveComponent Object Reference") (OtherBodyIndex :type Integer) (bFromSweep :type Boolean) (SweepResult :type "HitResult Structure (by ref)"))
  (`self.UnlockGate`))

(fn `UserConstructionScript`)