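; Game mode for The Witch Trials that picks a random spawn point on request.
; GetASpawnPoint finds a SpawnLocations actor, reads its location array and passes a random element to SpawnSpot.
; The debug print re-rolls the random index, so it can differ from the one used.
; The game mode's own GetSpawnLocationArray is an empty stub, and BeginPlay only calls the parent.
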(event `self.ReceiveBeginPlay`
  (`parent.ReceiveBeginPlay`))

(event `self.GetASpawnPoint`
  (bind _returnvalue (`GameplayStatics.GetActorOfClass` "/Game/Blueprints/SpawnLocations.SpawnLocations_C"))
  (bind _finallocations (`self.Get Spawn Location Array` _returnvalue))
  (bind _returnvalue_2 (`KismetMathLibrary.RandomInteger` (`KismetArrayLibrary.Array_Length` _finallocations)))
  (`self.SpawnSpot` (`|GetArrayItem` _finallocations _returnvalue_2))
  (`KismetSystemLibrary.PrintString` (`KismetStringLibrary.Conv_IntToString` _returnvalue_2)))

(fn `Get Spawn Location Array`
  (returns (FinalLocations :type "Array of Vector Structure"))
  (return))

(fn `UserConstructionScript`)