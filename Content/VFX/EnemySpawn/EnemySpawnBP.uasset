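; Enemy spawn effect actor that plays a Niagara effect while a skeletal mesh rises into place, then spawns the real enemy.
; On BeginPlay the Raise timeline lerps the mesh's relative Z from a starting offset up to zero.
; When it finishes, the mesh is destroyed and, one tick later, BP_EnemyAI spawns slightly above the actor's transform, followed by a debug print.
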(event `self.ReceiveBeginPlay`
  (bind (_returnvalue_location _returnvalue_rotation _returnvalue_scale) (`KismetMathLibrary.BreakTransform` (`self.GetTransform`)))
  (`ActorComponent.Activate` (`self.Niagara`) false)
  (bind (_direction _raise) (`Timeline|Raise`)
    (:`Update`
      (`SceneComponent.K2_SetRelativeLocation` (`self.SkeletalMesh`) (`KismetMathLibrary.MakeVector` 0.0 0.0 (`KismetMathLibrary.Lerp` (`self.StartingPos`) 0.0 _raise)) false false))
    (:`Finished`
      (`ActorComponent.K2_DestroyComponent` (`self.SkeletalMesh`))
      (`KismetSystemLibrary.DelayUntilNextTick`)
      (`|SpawnActorFromClass` "/Game/Blueprints/AI/BP_EnemyAI.BP_EnemyAI_C" (`KismetMathLibrary.MakeTransform` (+ _returnvalue_location (0.0 0.0 80.0)) _returnvalue_rotation _returnvalue_scale) "Undefined" "OverrideRootScale" null null)
      (`KismetSystemLibrary.PrintString` "Hello"))))

(fn `UserConstructionScript`)