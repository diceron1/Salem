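; Blowing-leaves VFX actor that aligns a Niagara leaf effect with the global wind.
; The construction script assigns the LeafVFX system to the Leaves component.
; Tick writes ColorChange to custom primitive data and polls MPC_wind for strength and direction.
; When either changes, it offsets Leaves along the wind and downward, rotates it to the wind direction and reshapes its scale by strength.
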(event `self.ReceiveBeginPlay`)

(event `self.ReceiveTick`
  (params (DeltaSeconds :type "Float (single-precision)"))
  (bind _windstrength (`self.windStrength`))
  (bind _leaves (`self.leaves`))
  (bind _returnvalue (`KismetMathLibrary.FClamp` (/ 1.0 (`self.windStrength`))))
  (`PrimitiveComponent.SetCustomPrimitiveDataFloat` (`self.leaves`) 0 (`self.colorChange`))
  (`/Engine/EditorBlueprintResources/StandardMacros.DoOnce` false :!label _label
    (:`Completed`
      (bind _returnvalue_2 (`KismetMaterialLibrary.GetScalarParameterValue` "/Game/Environment/materials/MPC_wind.MPC_wind" "windStrength"))
      (bind _returnvalue_3 (`KismetMaterialLibrary.GetVectorParameterValue` "/Game/Environment/materials/MPC_wind.MPC_wind" "windDirection"))
      (if (or (!= _returnvalue_3 (`self.windDirection`)) (!= _returnvalue_2 (`self.windStrength`)))
        (set `self.windStrength` _returnvalue_2)
        (bind _output_get (set `self.windDirection` _returnvalue_3))
        (bind (_returnvalue_x _returnvalue_y) (`KismetMathLibrary.BreakVector` (* (`KismetMathLibrary.Conv_LinearColorToVector` _output_get) (* _windstrength 45.0))))
        (`SceneComponent.K2_SetRelativeLocation` _leaves (`KismetMathLibrary.MakeVector` _returnvalue_x _returnvalue_y (* (`KismetMathLibrary.MultiplyMultiply_FloatFloat` (* _windstrength 1.75) 1.8) -1.0)) false false)
        ;[1 1 1] adjust XYZ scale
        (`SceneComponent.SetRelativeScale3D` _leaves (`KismetMathLibrary.MakeVector` (`KismetMathLibrary.Lerp` 1.25 1.0 _returnvalue) (`KismetMathLibrary.Lerp` 0.75 1.0 _returnvalue) (`KismetMathLibrary.Lerp` 0.8 1.6 _returnvalue)))
        (`SceneComponent.K2_SetRelativeRotation` (`self.leaves`) (`KismetMathLibrary.MakeRotFromX` (`KismetMathLibrary.Conv_LinearColorToVector` (`self.windDirection`))) false false)
        (goto _label :!via `Reset`)
        (else
          (goto _label :!via `Reset`))))))

(fn `UserConstructionScript`
  (`NiagaraComponent.SetAsset` (`self.leaves`) (`self.leafVFX`) true))