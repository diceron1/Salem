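; Wind control actor whose displacement from its construction-time location drives environment wind and color change through the MPC_wind parameter collection.
; On Tick, horizontal offset sets wind strength and direction, while vertical offset sets a clamped color-change value.
; A WindVector arrow visualizes the offset through orientation, length and green-to-red color.
; Changed values are written to the collection; per-actor tree and leaf recoloring is left unconnected.
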(event `self.ReceiveTick`
  (params (DeltaSeconds :type "Float (single-precision)"))
  (bind _returnvalue (`self.K2_GetActorLocation`))
  (bind (_returnvalue_x _returnvalue_y) (`KismetMathLibrary.BreakVector` (`self.K2_GetActorLocation`)))
  (bind (_returnvalue_x_2 _returnvalue_y_2 _returnvalue_z) (`KismetMathLibrary.BreakVector` (`self.K2_GetActorLocation`)))
  (bind (_startlocation_x _startlocation_y _startlocation_z) (`KismetMathLibrary.BreakVector` (`self.startLocation`)))
  (bind _windvector (`self.windVector`))
  (bind _windstrength (`self.windStrength`))
  (bind _winddirection (`self.windDirection`))
  (bind _olddirection (`self.oldDirection`))
  (bind _colorchange (`self.colorChange`))
  (bind _startlocation (`self.startLocation`))
  (bind (_startlocation_x_2 _startlocation_y_2) (`KismetMathLibrary.BreakVector` (`self.startLocation`)))
  (bind _returnvalue_2 (`KismetMathLibrary.Vector_Distance` (`KismetMathLibrary.MakeVector` (.x _startlocation) (.y _startlocation)) (`KismetMathLibrary.MakeVector` (.x _returnvalue) (.y _returnvalue))))
  (`|ExecutionSequence`
    (:`then_0`
      (`/Engine/EditorBlueprintResources/StandardMacros.DoOnce` (not (`self.moveControlEnabled?`)) :!label _label
        (:`Completed`
          ;[1 1 1] has position changed?
          (if (!= (`self.oldLocation`) (`self.K2_GetActorLocation`))
            ;[1 1 1] test Color Change
            (set `self.colorChange` (`KismetMathLibrary.FClamp` (/ (`KismetMathLibrary.Vector_Distance` (`KismetMathLibrary.MakeVector` _returnvalue_x_2 _returnvalue_y_2 _startlocation_z) (`KismetMathLibrary.MakeVector` _returnvalue_x_2 _returnvalue_y_2 _returnvalue_z)) 500.0)))
            ;[1 1 1] adjust arrow location/orientation; update arrow visual; get wind strength
            (`SceneComponent.K2_SetWorldLocationAndRotation` _windvector (`KismetMathLibrary.MakeVector` (.x _startlocation) (.y _startlocation) 100.0) (`KismetMathLibrary.FindLookAtRotation` _startlocation _returnvalue) false false)
            (`ArrowComponent.SetArrowColor` _windvector (`KismetMathLibrary.LinearColorLerp` (struct :`R` 0.091339 :`G` 1.0 :`A` 1.0) (struct :`R` 1.0 :`B` 0.03269 :`A` 1.0) (`KismetMathLibrary.NormalizeToRange` _returnvalue_2 0.0 500.0)))
            (`SceneComponent.SetRelativeScale3D` _windvector (`KismetMathLibrary.MakeVector` (/ (`KismetMathLibrary.Vector_Distance` _startlocation _returnvalue) 100.0) 1.0 1.0))
            (set `self.windStrength` (/ _returnvalue_2 100.0))
            ;[1 1 1] determine wind direction
            (set `self.windDirection` (`KismetMathLibrary.GetForwardVector` (`KismetMathLibrary.FindLookAtRotation` (`KismetMathLibrary.MakeVector` _startlocation_x_2 _startlocation_y_2) (`KismetMathLibrary.MakeVector` _returnvalue_x _returnvalue_y))))
            (goto _label :!via `Reset`)
            (else
              (goto _label :!via `Reset`))))))
    (:`then_1`
      ;[1 1 1] change color (?)
      (if (!= _colorchange (`self.colorOld`))
        (set `self.colorOld` _colorchange)
        (`KismetMaterialLibrary.SetScalarParameterValue` "/Game/Environment/materials/MPC_wind.MPC_wind" "colorChange" _colorchange)))
    (:`then_2`
      ;[1 1 1] set strength
      (if (!= _windstrength (`self.oldStrength`))
        (set `self.oldStrength` _windstrength)
        (`KismetMaterialLibrary.SetScalarParameterValue` "/Game/Environment/materials/MPC_wind.MPC_wind" "windStrength" _windstrength)))
    (:`then_3`
      ;[1 1 1] set direction
      (if (!= _winddirection _olddirection)
        (set `self.oldDirection` _olddirection)
        (`KismetMaterialLibrary.SetVectorParameterValue` "/Game/Environment/materials/MPC_wind.MPC_wind" "windDirection" (`KismetMathLibrary.Conv_VectorToLinearColor` _winddirection))))))

(fn `UserConstructionScript`
  (bind _output_get (set `self.startLocation` (`self.K2_GetActorLocation`)))
  (set `self.oldLocation` _output_get))