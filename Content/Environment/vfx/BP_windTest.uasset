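; BP_windTest is a test control actor that turns its displacement from its construction location into wind and tree color.
; Each tick, horizontal offset sets windStrength and windDirection in MPC_wind, while an arrow component visualizes the offset through rotation, length and green-to-red color.
; Vertical distance becomes a clamped color value, pushed only on change to tree-tagged static meshes through Custom Primitive Data and to BP_blowingLeafControl actors.
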(event `self.ReceiveBeginPlay`)

(event `self.ReceiveTick`
  (params (DeltaSeconds :type "Float (single-precision)"))
  (bind _returnvalue (`self.K2_GetActorLocation`))
  (bind (_returnvalue_x _returnvalue_y _returnvalue_z) (`KismetMathLibrary.BreakVector` (`self.K2_GetActorLocation`)))
  (bind (_returnvalue_x_2 _returnvalue_y_2) (`KismetMathLibrary.BreakVector` (`self.K2_GetActorLocation`)))
  (bind (_startlocation_x _startlocation_y _startlocation_z) (`KismetMathLibrary.BreakVector` (`self.startLocation`)))
  (bind _windvector (`self.windVector`))
  (bind _colorchange (`self.colorChange`))
  (bind _startlocation (`self.startLocation`))
  (bind (_startlocation_x_2 _startlocation_y_2) (`KismetMathLibrary.BreakVector` (`self.startLocation`)))
  (bind _returnvalue_2 (`KismetMathLibrary.Vector_Distance` (`KismetMathLibrary.MakeVector` (.x _startlocation) (.y _startlocation)) (`KismetMathLibrary.MakeVector` (.x _returnvalue) (.y _returnvalue))))
  (`|ExecutionSequence`
    (:`then_0`
      (set `self.colorChange` (`KismetMathLibrary.FClamp` (/ (`KismetMathLibrary.Vector_Distance` (`KismetMathLibrary.MakeVector` _returnvalue_x _returnvalue_y _startlocation_z) (`KismetMathLibrary.MakeVector` _returnvalue_x _returnvalue_y _returnvalue_z)) 500.0)))
      (`SceneComponent.K2_SetWorldLocationAndRotation` _windvector (`KismetMathLibrary.MakeVector` (.x _startlocation) (.y _startlocation) 100.0) (`KismetMathLibrary.FindLookAtRotation` _startlocation _returnvalue) false false)
      (`ArrowComponent.SetArrowColor` _windvector (`KismetMathLibrary.LinearColorLerp` (struct :`R` 0.091339 :`G` 1.0 :`A` 1.0) (struct :`R` 1.0 :`B` 0.03269 :`A` 1.0) (`KismetMathLibrary.NormalizeToRange` _returnvalue_2 0.0 500.0)))
      (`SceneComponent.SetRelativeScale3D` _windvector (`KismetMathLibrary.MakeVector` (/ (`KismetMathLibrary.Vector_Distance` _startlocation _returnvalue) 100.0) 1.0 1.0))
      (`KismetMaterialLibrary.SetScalarParameterValue` "/Game/Environment/materials/MPC_wind.MPC_wind" "windStrength" (/ _returnvalue_2 100.0))
      (`KismetMaterialLibrary.SetVectorParameterValue` "/Game/Environment/materials/MPC_wind.MPC_wind" "windDirection" (`KismetMathLibrary.Conv_VectorToLinearColor` (`KismetMathLibrary.GetForwardVector` (`KismetMathLibrary.FindLookAtRotation` (`KismetMathLibrary.MakeVector` _startlocation_x_2 _startlocation_y_2) (`KismetMathLibrary.MakeVector` _returnvalue_x_2 _returnvalue_y_2))))))
    (:`then_1`
      (if (!= _colorchange (`self.colorOld`))
        (set `self.colorOld` _colorchange)
        ;[1 1 1] change tree color
        (bind _outactors (`GameplayStatics.GetAllActorsOfClassWithTag` "/Script/Engine.StaticMeshActor" "tree"))
        (for _array_element _outactors
          (`PrimitiveComponent.SetCustomPrimitiveDataFloat` (`StaticMeshActor.StaticMeshComponent` _array_element) 0 (`self.colorChange`)))
        ;[1 1 1] change blowing leaf color
        (bind _outactors_2 (`GameplayStatics.GetAllActorsOfClassWithTag` "/Game/Environment/vfx/BP_blowingLeafControl.BP_blowingLeafControl_C" "tree"))
        (for _array_element_2 _outactors_2
          (set `/Game/Environment/vfx/BP_blowingLeafControl.colorChange` (`self.colorChange`) _array_element_2))))))

(fn `UserConstructionScript`
  (set `self.startLocation` (`self.K2_GetActorLocation`)))