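; BP_cross is a configurable environment prop that assembles a thick, thin or stake cross from modular meshes.
; The construction script sets the vertical post, then adds a horizontal post and optional circle where the variants allow, plus ties for stake crosses.
; Ticking Randomize runs RandomizeConfig, which picks valid variants and limit-bounded transform jitter, then clears the flag so the result stays hand-editable.
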(fn `randomizeConfig`
  (bind _randomlocationlimit (`self.randomLocationLimit`))
  (bind _randomrotationlimit (`self.randomRotationLimit`))
  (bind _randomscalelimit (`self.randomScaleLimit`))
  (bind _crosstype (`self.crossType`))
  (bind _returnvalue (* _randomlocationlimit -1.0))
  (bind _returnvalue_2 (* _randomrotationlimit -1.0))
  (bind _returnvalue_3 (* _randomscalelimit -1.0))
  (bind _returnvalue_4 (/ (`self.randomRotationLimit`) 2.0))
  (bind _returnvalue_5 (/ (`self.randomScaleLimit`) 2.0))
  (bind _returnvalue_6 (/ (`self.randomLocationLimit`) 2.0))
  (bind _returnvalue_7 (/ (`self.randomLocationLimit`) 4.0))
  (bind _returnvalue_8 (`KismetMathLibrary.RandomFloatInRange` _returnvalue_3 _randomscalelimit))
  (bind _returnvalue_9 (* _returnvalue_4 -1.0))
  (bind _returnvalue_10 (* _returnvalue_6 -1.0))
  (`|ExecutionSequence`
    (:`then_0`
      ;[1 1 1] select baseType and vertical variant
      ;;[0.2778 0.06791 1] change crossType
      (bind _output_get (set `self.crossType` (`KismetMathLibrary.RandomIntegerInRange` 1 3)))
      ;;[0.2778 0.06791 1] change verticalVariant
      (set `self.verticalVariant` (`KismetMathLibrary.RandomIntegerInRange` 1 (`KismetMathLibrary.SelectInt` 5 2 (== _output_get 1)))))
    (:`then_1`
      ;[1 1 1] change horizontal variant
      (set `self.horizontalVariant` (`KismetMathLibrary.RandomIntegerInRange` 1 (select `int` (- (`self.crossType`) 1) :`0` (`KismetMathLibrary.SelectInt` 3 2 (== (`self.verticalVariant`) 4)) :`1` 4 :`2` 3))))
    (:`then_2`
      ;[1 1 1] change circle variant
      (set `self.circleVariant` (`KismetMathLibrary.RandomInteger` 3)))
    (:`then_3`
      ;[1 1 1] randomize baseTransform
      (set `self.baseTransform` (`KismetMathLibrary.MakeTransform` (`KismetMathLibrary.MakeVector` (`KismetMathLibrary.RandomFloatInRange` _returnvalue _randomlocationlimit) (`KismetMathLibrary.RandomFloatInRange` _returnvalue _randomlocationlimit) (`KismetMathLibrary.RandomFloatInRange` _returnvalue _randomlocationlimit)) (`KismetMathLibrary.MakeRotator` (`KismetMathLibrary.RandomFloatInRange` _returnvalue_2 _randomrotationlimit) (`KismetMathLibrary.RandomFloatInRange` _returnvalue_2 _randomrotationlimit) (`KismetMathLibrary.RandomFloatInRange` _returnvalue_2 _randomrotationlimit)) (+ (`KismetMathLibrary.SelectVector` (`KismetMathLibrary.Conv_DoubleToVector` _returnvalue_8) (`KismetMathLibrary.MakeVector` _returnvalue_8 (`KismetMathLibrary.RandomFloatInRange` _returnvalue_3 _randomscalelimit) (`KismetMathLibrary.RandomFloatInRange` _returnvalue_3 _randomscalelimit)) (`self.uniformRandomizedScale`)) (1.0 1.0 1.0)))))
    (:`then_4`
      ;[1 0.7602 0.2323] is able to translate/rotate hPost?
      (if (or (and (== _crosstype 1) (== (`self.verticalVariant`) 4)) (> _crosstype 1))
        ;[1 1 1] randomize horizontal Location&Rotation
        (set `self.horizontalTransform` (`KismetMathLibrary.MakeTransform` (`KismetMathLibrary.MakeVector` (`KismetMathLibrary.RandomFloatInRange` _returnvalue_10 _returnvalue_6) 0.0 (`KismetMathLibrary.RandomFloatInRange` _returnvalue_10 _returnvalue_6)) (`KismetMathLibrary.MakeRotator` 0.0 (`KismetMathLibrary.RandomFloatInRange` _returnvalue_9 _returnvalue_4) (`KismetMathLibrary.RandomFloatInRange` _returnvalue_9 _returnvalue_4)) (`KismetMathLibrary.MakeVector` (* (`KismetMathLibrary.SelectFloat` 1.0 (+ (`KismetMathLibrary.RandomFloatInRange` (* _returnvalue_5 -1.0) _returnvalue_5) 1.0) (`self.uniformRandomizedScale`)) (`KismetMathLibrary.SelectFloat` 1.0 -1.0 (`KismetMathLibrary.RandomBool`))) 1.0 1.0)))
        ;[1 1 1] randomize circle offset
        (set `self.circleVerticalOffset` (`KismetMathLibrary.RandomFloatInRange` (* _returnvalue_7 -1.0) _returnvalue_7))
        (else
          ;[1 1 1] zeroOut if transform is invalid
          (set `self.horizontalTransform` (`KismetMathLibrary.MakeTransform` (0.0 0.0 0.0)))
          ;[1 1 1] zeroOut circle offset
          (set `self.circleVerticalOffset` 0.0))))
    (:`then_6`
      ;[1 1 1] turn off randomize for editability
      (set `self.randomize` false)
      (return))))

(fn `UserConstructionScript`
  (bind _base (`self.base`))
  (bind _verticalvariant (`self.verticalVariant`))
  (bind _horizontalvariant (`self.horizontalVariant`))
  (bind _horizontaltransform (`self.horizontalTransform`))
  (bind _horizontaltransform_2 (`self.horizontalTransform`))
  (bind _horizontaltransform_3 (`self.horizontalTransform`))
  (bind _horizontaltransform_4 (`self.horizontalTransform`))
  (bind _verticalvariant_2 (`self.verticalVariant`))
  (bind _crosstype (`self.crossType`))
  (bind _returnvalue (- _horizontalvariant 1))
  (bind _returnvalue_2 (== (`self.circleVariant`) 1))
  (bind _returnvalue_3 (== _verticalvariant_2 1))
  (bind _returnvalue_4 (`KismetMathLibrary.Clamp` _returnvalue 0 2))
  (if (`self.randomize`)
    (`self.randomizeConfig`))
  (`|ExecutionSequence`
    (:`then_0`
      ;[1 1 1] set verticalPost/baseCross
      (`StaticMeshComponent.SetStaticMesh` _base (select `int` (- (`self.crossType`) 1) :`0` (select `int` (- _verticalvariant_2 1) :`0` "/Game/Environment/meshes/cross/SM_cross_thick_01.SM_cross_thick_01" :`1` "/Game/Environment/meshes/cross/components/SM_cross_thick_02_v_01.SM_cross_thick_02_v_01" :`2` "/Game/Environment/meshes/cross/components/SM_cross_thick_02_v_02.SM_cross_thick_02_v_02" :`3` "/Game/Environment/meshes/cross/components/SM_cross_thick_03_v.SM_cross_thick_03_v" :`4` "/Game/Environment/meshes/cross/SM_cross_thick_04.SM_cross_thick_04" :!type "StaticMesh Object Reference") :`1` (select `bool` _returnvalue_3 :`false` "/Game/Environment/meshes/cross/components/SM_cross_thin_v_02.SM_cross_thin_v_02" :`true` "/Game/Environment/meshes/cross/components/SM_cross_thin_v_01.SM_cross_thin_v_01" :!type "StaticMesh Object Reference") :`2` (select `bool` _returnvalue_3 :`false` "/Game/Environment/meshes/cross/components/SM_cross_stake_v_02.SM_cross_stake_v_02" :`true` "/Game/Environment/meshes/cross/components/SM_cross_stake_v_01.SM_cross_stake_v_01" :!type "StaticMesh Object Reference")))
      (`SceneComponent.K2_SetRelativeTransform` _base (`self.baseTransform`) false false))
    (:`then_1`
      ;[1 0.7602 0.2323] prevent hPost creation if using thick_01 or thick_04
      (if (`KismetMathLibrary.BooleanNAND` (not (`KismetMathLibrary.InRange_IntInt` (`self.verticalVariant`) 2 4)) (== (`self.crossType`) 1))
        ;[1 1 1] build hPost
        (bind _returnvalue_5 (`AddComponent|NODE_AddStaticMeshComponent-0` :`RelativeTransform` (`KismetMathLibrary.MakeTransform` (0.0 0.0 -65.0))))
        (`StaticMeshComponent.SetStaticMesh` _returnvalue_5 (select `int` (- (`self.crossType`) 1) :`0` (select `bool` (== (`self.verticalVariant`) 4) :`false` (select `bool` (== _horizontalvariant 1) :`false` "/Game/Environment/meshes/cross/components/SM_cross_thick_02_h_02.SM_cross_thick_02_h_02" :`true` "/Game/Environment/meshes/cross/components/SM_cross_thick_02_h_01.SM_cross_thick_02_h_01" :!type "StaticMesh Object Reference") :`true` (select `int` _returnvalue_4 :`0` "/Game/Environment/meshes/cross/components/SM_cross_thick_03_h_01.SM_cross_thick_03_h_01" :`1` "/Game/Environment/meshes/cross/components/SM_cross_thick_03_h_02.SM_cross_thick_03_h_02" :`2` "/Game/Environment/meshes/cross/components/SM_cross_thick_03_h_03.SM_cross_thick_03_h_03" :!type "StaticMesh Object Reference")) :`1` (select `int` _returnvalue :`0` "/Game/Environment/meshes/cross/components/SM_cross_thin_h_01.SM_cross_thin_h_01" :`1` "/Game/Environment/meshes/cross/components/SM_cross_thin_h_02.SM_cross_thin_h_02" :`2` "/Game/Environment/meshes/cross/components/SM_cross_thin_h_03.SM_cross_thin_h_03" :`3` "/Game/Environment/meshes/cross/components/SM_cross_thin_h_04.SM_cross_thin_h_04" :!type "StaticMesh Object Reference") :`2` (select `int` _returnvalue_4 :`0` "/Game/Environment/meshes/cross/components/SM_cross_stake_h_01.SM_cross_stake_h_01" :`1` "/Game/Environment/meshes/cross/components/SM_cross_stake_h_02.SM_cross_stake_h_02" :`2` "/Game/Environment/meshes/cross/components/SM_cross_stake_h_03.SM_cross_stake_h_03" :!type "StaticMesh Object Reference")))
        (`SceneComponent.K2_AttachToComponent` _returnvalue_5 (`self.hPostParent`) "None" "KeepRelative" "KeepRelative" "KeepRelative" true)
        ;[1 1 1] build stake hPostTie
        ;;[1 0.7602 0.2323] is stakeType?
        (if (== (`self.crossType`) 3)
          (bind _returnvalue_6 (`AddComponent|NODE_AddStaticMeshComponent-2` :`RelativeTransform` (`KismetMathLibrary.MakeTransform` (0.0 0.0 -65.0))))
          (`SceneComponent.K2_AttachToComponent` _returnvalue_6 (`self.hTieParent`) "None" "KeepRelative" "KeepRelative" "KeepRelative" true)
          ;[1 1 1] set hPost Parent Transform
          (`SceneComponent.K2_SetRelativeTransform` (`self.hPostParent`) (`KismetMathLibrary.MakeTransform` (`KismetMathLibrary.MakeVector` (.x (.location _horizontaltransform_4)) (.y (.location _horizontaltransform_4)) (+ (.z (.location _horizontaltransform_4)) 65.0)) (.rotation _horizontaltransform_4) (.scale _horizontaltransform_4)) false false)
          ;[1 1 1] set hTieParent transform
          (`SceneComponent.K2_SetRelativeTransform` (`self.hTieParent`) (`KismetMathLibrary.MakeTransform` (`KismetMathLibrary.MakeVector` 0.0 0.0 (+ (.z (.location _horizontaltransform)) 65.0)) (`KismetMathLibrary.MakeRotator` 0.0 (/ (.pitch (.rotation _horizontaltransform)) 2.0) (.yaw (.rotation _horizontaltransform)))) false false))))
    (:`then_2`
      ;[1 0.7602 0.2323] are circles possible?
      (if (and (> (`self.circleVariant`) 0) (or (== _crosstype 3) (and (== _crosstype 1) (or (== _verticalvariant 1) (and (== _verticalvariant 2) (== (`self.horizontalVariant`) 1))))))
        ;[1 1 1] build circle
        (bind _returnvalue_7 (`AddComponent|NODE_AddStaticMeshComponent-1` :`RelativeTransform` (`KismetMathLibrary.MakeTransform` (`KismetMathLibrary.MakeVector` 0.0 0.0 (+ (.z (.location _horizontaltransform_3)) (`self.circleVerticalOffset`))) (`KismetMathLibrary.MakeRotator` 0.0 0.0 (.yaw (.rotation _horizontaltransform_3))))))
        (`StaticMeshComponent.SetStaticMesh` _returnvalue_7 (select `bool` (== (`self.crossType`) 1) :`false` (select `bool` _returnvalue_2 :`false` "/Game/Environment/meshes/cross/components/SM_cross_stake_circ_02.SM_cross_stake_circ_02" :`true` "/Game/Environment/meshes/cross/components/SM_cross_stake_circ_01.SM_cross_stake_circ_01" :!type "StaticMesh Object Reference") :`true` (select `bool` (== (`self.verticalVariant`) 1) :`false` (select `bool` _returnvalue_2 :`false` "/Game/Environment/meshes/cross/components/SM_cross_thick_02_circ_02.SM_cross_thick_02_circ_02" :`true` "/Game/Environment/meshes/cross/components/SM_cross_thick_02_circ_01.SM_cross_thick_02_circ_01" :!type "StaticMesh Object Reference") :`true` (select `bool` _returnvalue_2 :`false` "/Game/Environment/meshes/cross/components/SM_cross_thick_01_circ_02.SM_cross_thick_01_circ_02" :`true` "/Game/Environment/meshes/cross/components/SM_cross_thick_01_circ_01.SM_cross_thick_01_circ_01" :!type "StaticMesh Object Reference"))))
        (`SceneComponent.K2_AttachToComponent` _returnvalue_7 (`self.base`) "None" "KeepRelative" "KeepRelative" "KeepRelative" true)
        ;[1 1 1] build stake circleTie
        ;;[1 0.7602 0.2323] is stakeType?
        (if (== (`self.crossType`) 3)
          (bind _returnvalue_8 (`AddComponent|NODE_AddStaticMeshComponent-3` :`RelativeTransform` (`KismetMathLibrary.MakeTransform` (`KismetMathLibrary.MakeVector` 0.0 0.0 (+ (.z (.location _horizontaltransform_2)) (`self.circleVerticalOffset`))) (`KismetMathLibrary.MakeRotator` 0.0 0.0 (.yaw (.rotation _horizontaltransform_2))))))
          (`SceneComponent.K2_AttachToComponent` _returnvalue_8 (`self.base`) "None" "KeepRelative" "KeepRelative" "KeepRelative" true))))))