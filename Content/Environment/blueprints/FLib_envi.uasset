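; FLib_envi is an environment function library that sets up mesh materials from named presets or custom parameter sets.
; AssignMaterials creates a dynamic instance for every material slot across a mesh array, consuming names from one flat list via a running index.
; Names like "customN" select entry N of a custom array when valid; others are DT_matParams row names.
; AssignMatParams pushes the resolved struct's map switches, textures, colors and scalars into each instance.
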(fn `assignMaterials`
  (params (meshArray :type "Array of MeshComponent Object Reference") (matArray :type "Array of Name") (customArray :type "Array of /Game/Environment/blueprints/ST_baseMatParams Structure (by ref)"))
  (locals (L_bulkIndex :type Integer :default 0) (`L_custom?` :type Boolean) (L_customParam :type "/Game/Environment/blueprints/ST_baseMatParams Structure"))
  (bind _customarray (`local.customArray`))
  (bind _output (`|GetArrayItem` (`local.matArray`) (`local.L_bulkIndex`)))
  (bind _returnvalue (`KismetStringLibrary.Conv_NameToString` _output))
  (bind _returnvalue_2 (`KismetStringLibrary.Conv_StringToInt` (`KismetStringLibrary.RightChop` _returnvalue 5)))
  (for _array_element meshArray
    (for (_ _array_index) (`MeshComponent.GetMaterials` _array_element)
      (set `local.L_custom?` false)
      (set `local.L_customParam` (struct))
      (bind _returnvalue_3 (`PrimitiveComponent.CreateDynamicMaterialInstance` _array_element _array_index null "None"))
      ;[1 1 1] attempt custom param?
      (if (`KismetStringLibrary.StartsWith` _returnvalue "custom")
        ;[1 1 1] set custom param if possible
        (bind _output_get (set `local.L_custom?` (`KismetArrayLibrary.Array_IsValidIndex` _customarray _returnvalue_2)))
        (if _output_get
          (set `local.L_customParam` (`|GetArrayItem` _customarray _returnvalue_2))))
      (`self.assignMatParams` _returnvalue_3 _output (`local.L_custom?`) (`local.L_customParam`))
      (`/Engine/EditorBlueprintResources/StandardMacros.IncrementInt` (`local.L_bulkIndex`)))))

(fn `assignMatParams`
  (params (materialInstance :type "MaterialInstanceDynamic Object Reference") (presetName :type Name) (`useCustom?` :type Boolean) (customParams :type "/Game/Environment/blueprints/ST_baseMatParams Structure"))
  (locals (L_matParams :type "/Game/Environment/blueprints/ST_baseMatParams Structure"))
  (bind _materialinstance (`local.materialInstance`))
  (bind _materialinstance_2 (`local.materialInstance`))
  (bind _materialinstance_3 (`local.materialInstance`))
  (bind _materialinstance_4 (`local.materialInstance`))
  (bind (_hascolormap _blendcolor _invertcolor _hasmergedmap _hasroughmap _hasambientmap _hasnormalmap _hasemissivemap _hasopacitymap _hasrefractionmap _mapcolor _color _brightness _blacklevel _newcolor) (break `/Game/Environment/blueprints/ST_baseMatParams` (`local.L_matParams`)))
  (bind (_hascolormap_2 _blendcolor_2 _invertcolor_2 _hasmergedmap_2 _hasroughmap_2 _hasambientmap_2 _hasnormalmap_2 _hasemissivemap_2 _hasopacitymap_2 _hasrefractionmap_2 _mapcolor_2 _color_2 _brightness_2 _blacklevel_2 _newcolor_2 _mapmerged _mapmetal _metalness _maprough _roughness _mapambient) (break `/Game/Environment/blueprints/ST_baseMatParams` (`local.L_matParams`)))
  (bind (_hascolormap_3 _blendcolor_3 _invertcolor_3 _hasmergedmap_3 _hasroughmap_3 _hasambientmap_3 _hasnormalmap_3 _hasemissivemap_3 _hasopacitymap_3 _hasrefractionmap_3 _mapcolor_3 _color_3 _brightness_3 _blacklevel_3 _newcolor_3 _mapmerged_2 _mapmetal_2 _metalness_2 _maprough_2 _roughness_2 _mapambient_2 _mapnormal _mapemissive _emissive _mapopacity _opacity _maprefraction _refraction) (break `/Game/Environment/blueprints/ST_baseMatParams` (`local.L_matParams`)))
  (bind (_hascolormap_4 _blendcolor_4 _invertcolor_4 _hasmergedmap_4 _hasroughmap_4 _hasambientmap_4 _hasnormalmap_4 _hasemissivemap_4 _hasopacitymap_4 _hasrefractionmap_4) (break `/Game/Environment/blueprints/ST_baseMatParams` (`local.L_matParams`)))
  ;[1 1 1] establish params to use
  (if `useCustom?`
    (set `local.L_matParams` customParams)
    (else
      (bind _returnvalue (`|GetDataTableRow` "/Game/Environment/blueprints/DT_matParams.DT_matParams" presetName)
        (:`then`
          (set `local.L_matParams` _returnvalue))
        (:`RowNotFound`
          _))))
  (`|ExecutionSequence`
    (:`then_0`
      ;[1 1 1] set switch params
      (`MaterialInstanceDynamic.SetScalarParameterValue` _materialinstance_3 "hasColorMap" _hascolormap_4)
      (`MaterialInstanceDynamic.SetScalarParameterValue` _materialinstance_3 "blendColor" _blendcolor_4)
      (`MaterialInstanceDynamic.SetScalarParameterValue` _materialinstance_3 "invertColor" _invertcolor_4)
      (`MaterialInstanceDynamic.SetScalarParameterValue` _materialinstance_3 "hasMergedMap" _hasmergedmap_4)
      (`MaterialInstanceDynamic.SetScalarParameterValue` _materialinstance_3 "hasRoughMap" _hasroughmap_4)
      (`MaterialInstanceDynamic.SetScalarParameterValue` _materialinstance_3 "hasAmbientMap" _hasambientmap_4)
      (`MaterialInstanceDynamic.SetScalarParameterValue` _materialinstance_3 "hasNormalMap" _hasnormalmap_4)
      (`MaterialInstanceDynamic.SetScalarParameterValue` _materialinstance_3 "hasEmissiveMap" _hasemissivemap_4)
      (`MaterialInstanceDynamic.SetScalarParameterValue` _materialinstance_3 "hasOpacityMap" _hasopacitymap_4)
      (`MaterialInstanceDynamic.SetScalarParameterValue` _materialinstance_3 "hasRefractionMap" _hasrefractionmap_4))
    (:`then_1`
      ;[1 1 1] set color params
      (`MaterialInstanceDynamic.SetTextureParameterValue` _materialinstance "mapColor" _mapcolor)
      (`MaterialInstanceDynamic.SetVectorParameterValue` _materialinstance "color" _color)
      (`MaterialInstanceDynamic.SetScalarParameterValue` _materialinstance "brightness" _brightness)
      (`MaterialInstanceDynamic.SetScalarParameterValue` _materialinstance "blackLevel" _blacklevel)
      (`MaterialInstanceDynamic.SetVectorParameterValue` _materialinstance "newColor" _newcolor))
    (:`then_2`
      ;[1 1 1] set merged or metal/rough/AO params
      (`MaterialInstanceDynamic.SetTextureParameterValue` _materialinstance_4 "mapMerged" _mapmerged)
      (`MaterialInstanceDynamic.SetTextureParameterValue` _materialinstance_4 "mapMetal" _mapmetal)
      (`MaterialInstanceDynamic.SetScalarParameterValue` _materialinstance_4 "metalness" _metalness)
      (`MaterialInstanceDynamic.SetTextureParameterValue` _materialinstance_4 "mapRough" _maprough)
      (`MaterialInstanceDynamic.SetScalarParameterValue` _materialinstance_4 "roughness" _roughness)
      (`MaterialInstanceDynamic.SetTextureParameterValue` _materialinstance_4 "mapAmbient" _mapambient))
    (:`then_3`
      ;[1 1 1] set misc params
      (`MaterialInstanceDynamic.SetTextureParameterValue` _materialinstance_2 "mapNormal" _mapnormal)
      (`MaterialInstanceDynamic.SetTextureParameterValue` _materialinstance_2 "mapEmissive" _mapemissive)
      (`MaterialInstanceDynamic.SetVectorParameterValue` _materialinstance_2 "emissive" _emissive)
      (`MaterialInstanceDynamic.SetTextureParameterValue` _materialinstance_2 "mapOpacity" _mapopacity)
      (`MaterialInstanceDynamic.SetScalarParameterValue` _materialinstance_2 "opacity" _opacity)
      (`MaterialInstanceDynamic.SetTextureParameterValue` _materialinstance_2 "mapRefraction" _maprefraction)
      (`MaterialInstanceDynamic.SetScalarParameterValue` _materialinstance_2 "refraction" _refraction))))