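; Modular mausoleum prop that assembles itself from static mesh pieces in the construction script, with a Randomize switch between two build functions.
; BuildStandard sets roof, door, handles, columns, crown, windows and decor from variables and mesh/transform arrays.
; BuildRandom rolls these choices unseeded, storing them in locals so handle and decor placement fit the chosen door and roof.
; A DoOnce loop-back can layer a second decor mesh.
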(fn `buildRandom`
  (locals (`L_flatRoof?` :type Boolean :default false) (L_doorType :type Integer :default 0) (`L_fancyHandle?` :type Boolean :default false) (L_columnType :type Integer :default 0) (L_columnLocY :type "Float (double-precision)" :default 0.0) (L_crownType :type Integer :default 0) (L_windowPosition :type Integer) (L_decorPosition :type Integer) (L_decorMesh :type "StaticMesh Object Reference") (L_decorType :type Integer :default 0))
  (bind _returnvalue (`KismetMathLibrary.RandomInteger` 3))
  (bind (_columnoffset_x _columnoffset_y) (`KismetMathLibrary.BreakVector2D` (`self.columnOffset`)))
  (bind (_columnoffset_x_2 _columnoffset_y_2) (`KismetMathLibrary.BreakVector2D` (`self.columnOffset`)))
  (bind (_crownoffset_x _crownoffset_y) (`KismetMathLibrary.BreakVector2D` (`self.crownOffset`)))
  (bind _l_flatroof_ (`local.L_flatRoof?`))
  (bind _l_decortype (`local.L_decorType`))
  (bind _returnvalue_2 (`KismetMathLibrary.SelectFloat` 0.9 1.0 _l_flatroof_))
  (bind _returnvalue_3 (== 0 (`local.L_doorType`)))
  (bind _returnvalue_4 (== (`local.L_decorPosition`) 1))
  (bind _returnvalue_5 (== (`local.L_doorType`) 0))
  (bind _returnvalue_6 (== _l_decortype 1))
  (bind _returnvalue_7 (select `int` _returnvalue :`0` -25.0 :`1` 25.0 :`2` 50.0))
  (bind _returnvalue_8 (`KismetMathLibrary.SelectFloat` 0.6 1.0 _returnvalue_5))
  (`|ExecutionSequence`
    (:`then_0`
      ;[1 1 1] change roof type
      ;;[0.2778 0.06791 1] remember selection
      (bind _output_get (set `local.L_flatRoof?` (`KismetMathLibrary.RandomBool`)))
      (`StaticMeshComponent.SetStaticMesh` (`self.roof`) (select `bool` _output_get :`false` "/Game/Environment/meshes/mausoleum/SM_maus_roofAngle.SM_maus_roofAngle" :`true` "/Game/Environment/meshes/mausoleum/SM_maus_roofFlat.SM_maus_roofFlat" :!type "StaticMesh Object Reference")))
    (:`then_1`
      ;[1 1 1] change doorType
      ;;[0.2778 0.06791 1] select doorType
      (bind _output_get_2 (set `local.L_doorType` (`KismetMathLibrary.RandomInteger` 3)))
      (`StaticMeshComponent.SetStaticMesh` (`self.door`) (select `int` _output_get_2 :`0` "/Game/Environment/meshes/mausoleum/SM_maus_door_01.SM_maus_door_01" :`1` "/Game/Environment/meshes/mausoleum/SM_maus_door_02.SM_maus_door_02" :`2` "/Game/Environment/meshes/mausoleum/SM_maus_door_03.SM_maus_door_03" :!type "StaticMesh Object Reference")))
    (:`then_2`
      ;[1 1 1] build doorHandle(s)
      ;;[0.1604 0.5721 1] build baseHandle
      ;;;[1 1 1] position baseHandle
      (bind _returnvalue_9 (`AddComponent|NODE_AddStaticMeshComponent-9` :`RelativeTransform` (`KismetMathLibrary.MakeTransform` (`KismetMathLibrary.MakeVector` (`KismetMathLibrary.SelectFloat` 5.0 -53.0 _returnvalue_3) 128.0 85.0))))
      ;;;[0.2778 0.06791 1] select handleType
      (bind _output_get_3 (set `local.L_fancyHandle?` (`KismetMathLibrary.RandomBool`)))
      ;;;[1 1 1] change handleMesh
      (`StaticMeshComponent.SetStaticMesh` _returnvalue_9 (select `bool` _output_get_3 :`false` "/Game/Environment/meshes/mausoleum/SM_maus_doorHandle_01.SM_maus_doorHandle_01" :`true` "/Game/Environment/meshes/mausoleum/SM_maus_doorHandle_02.SM_maus_doorHandle_02" :!type "StaticMesh Object Reference"))
      ;;[1 0.7602 0.2323] is doubleDoor?
      (if _returnvalue_3
        ;;[0.1604 0.5721 1] add secondHandle
        (bind _returnvalue_10 (`AddComponent|NODE_AddStaticMeshComponent-10` :`RelativeTransform` (`KismetMathLibrary.MakeTransform` (-5.0 128.0 85.0) (struct) (-1.0 1.0 1.0))))
        (`StaticMeshComponent.SetStaticMesh` _returnvalue_10 (select `bool` (`local.L_fancyHandle?`) :`false` "/Game/Environment/meshes/mausoleum/SM_maus_doorHandle_01.SM_maus_doorHandle_01" :`true` "/Game/Environment/meshes/mausoleum/SM_maus_doorHandle_02.SM_maus_doorHandle_02" :!type "StaticMesh Object Reference"))
        ;;[0.1604 0.5721 1] adjust lock to doubleDoor
        (`SceneComponent.K2_SetRelativeLocation` (`self.lock`) (-5.0 128.0 100.0) false false)))
    (:`then_3`
      ;[1 1 1] build columns
      ;;[0.2778 0.06791 1] select column type
      (bind _output_get_4 (set `local.L_columnType` (`KismetMathLibrary.RandomInteger` 3)))
      ;;[1 0.7602 0.2323] are columns enabled?
      (if (> _output_get_4 0)
        ;;[0.2778 0.06791 1] select forward offset
        (set `local.L_columnLocY` (`KismetMathLibrary.SelectFloat` 159.0 135.0 (`KismetMathLibrary.RandomBool`)))
        ;;[0.1604 0.5721 1] build 1st column
        ;;;[1 1 1] set column location
        (bind _returnvalue_11 (`AddComponent|NODE_AddStaticMeshComponent-11` :`RelativeTransform` (`KismetMathLibrary.MakeTransform` (`KismetMathLibrary.MakeVector` (+ _columnoffset_x_2 94.0) (+ _columnoffset_y_2 (`local.L_columnLocY`))))))
        ;;;[1 1 1] set column meshType
        (`StaticMeshComponent.SetStaticMesh` _returnvalue_11 (select `bool` (== (`local.L_columnType`) 2) :`false` "/Game/Environment/meshes/mausoleum/SM_maus_col_01.SM_maus_col_01" :`true` "/Game/Environment/meshes/mausoleum/SM_maus_col_02.SM_maus_col_02" :!type "StaticMesh Object Reference"))
        ;;[0.1604 0.5721 1] build 2nd column
        ;;;[1 1 1] set column location
        (bind _returnvalue_12 (`AddComponent|NODE_AddStaticMeshComponent-12` :`RelativeTransform` (`KismetMathLibrary.MakeTransform` (`KismetMathLibrary.MakeVector` (- -94.0 _columnoffset_x) (+ _columnoffset_y (`local.L_columnLocY`))))))
        ;;;[1 1 1] set column meshType
        (`StaticMeshComponent.SetStaticMesh` _returnvalue_12 (select `bool` (== (`local.L_columnType`) 2) :`false` "/Game/Environment/meshes/mausoleum/SM_maus_col_01.SM_maus_col_01" :`true` "/Game/Environment/meshes/mausoleum/SM_maus_col_02.SM_maus_col_02" :!type "StaticMesh Object Reference"))))
    (:`then_4`
      ;[1 1 1] build crown
      ;;[0.2778 0.06791 1] select crown type
      (bind _output_get_5 (set `local.L_crownType` (`KismetMathLibrary.RandomInteger` 4)))
      ;;[1 0.7602 0.2323] is crown enabled?
      (if (> _output_get_5 0)
        ;;[0.1604 0.5721 1] set location/scale
        (bind _returnvalue_13 (`AddComponent|NODE_AddStaticMeshComponent-13` :`RelativeTransform` (`KismetMathLibrary.MakeTransform` (`KismetMathLibrary.MakeVector` 0.0 (+ _crownoffset_x 165.0) (+ _crownoffset_y 290.0)) (struct) (`self.crownScale`))))
        ;;[0.1604 0.5721 1] change mesh type
        (`StaticMeshComponent.SetStaticMesh` _returnvalue_13 (select `int` (- (`local.L_crownType`) 1) :`0` "/Game/Environment/meshes/mausoleum/SM_maus_cap_01.SM_maus_cap_01" :`1` "/Game/Environment/meshes/mausoleum/SM_maus_cap_02.SM_maus_cap_02" :`2` "/Game/Environment/meshes/mausoleum/SM_maus_cap_03.SM_maus_cap_03" :!type "StaticMesh Object Reference"))))
    (:`then_5`
      ;[1 1 1] build windows
      ;;[0.2778 0.06791 1] select window position
      (bind _output_get_6 (set `local.L_windowPosition` (`KismetMathLibrary.RandomInteger` 4)))
      ;;[1 0.7602 0.2323] are windows enabled?
      (if (> _output_get_6 0)
        ;;[0.1604 0.5721 1] add single window
        ;;;[1 1 1] set mesh transform
        (bind _returnvalue_14 (`AddComponent|NODE_AddStaticMeshComponent-14` :`RelativeTransform` (select `int` (- (`local.L_windowPosition`) 1) :`0` (`KismetMathLibrary.MakeTransform` (`KismetMathLibrary.MakeVector` (select `int` _returnvalue :`0` -60.0 :`1` 0.0 :`2` 60.0) -131.0 140.0) (struct :`Yaw` 180.0)) :`1` (`KismetMathLibrary.MakeTransform` (`KismetMathLibrary.MakeVector` -158.0 _returnvalue_7 140.0) (struct :`Yaw` 90.0)) :`2` (`KismetMathLibrary.MakeTransform` (`KismetMathLibrary.MakeVector` 158.0 _returnvalue_7 140.0) (struct :`Yaw` -90.0)))))
        ;;;[1 1 1] set mesh type
        (`StaticMeshComponent.SetStaticMesh` _returnvalue_14 (select `bool` (`KismetMathLibrary.RandomBool`) :`false` "/Game/Environment/meshes/mausoleum/SM_maus_win_01.SM_maus_win_01" :`true` "/Game/Environment/meshes/mausoleum/SM_maus_win_02.SM_maus_win_02" :!type "StaticMesh Object Reference"))))
    (:`then_6`
      ;[1 1 1] build decor
      ;;[0.2778 0.06791 1] select decor position
      (bind _output_get_7 (set `local.L_decorPosition` (`KismetMathLibrary.RandomInteger` 3)))
      ;;[1 0.7602 0.2323] is decor enabled?
      (if (> _output_get_7 0)
        ;;[0.2778 0.06791 1] save decor type index
        (set `local.L_decorType` (`KismetMathLibrary.RandomIntegerInRange` (`KismetMathLibrary.SelectInt` 0 1 (and (== (`local.L_decorPosition`) 1) (not (`local.L_flatRoof?`)))) 3))
        ;;[0.2778 0.06791 1] select mesh
        (set `local.L_decorMesh` (select `int` (`local.L_decorType`) :`0` "/Game/Environment/meshes/mausoleum/SM_maus_dec_01.SM_maus_dec_01" :`1` "/Game/Environment/meshes/mausoleum/SM_maus_dec_02.SM_maus_dec_02" :`2` "/Game/Environment/meshes/mausoleum/SM_maus_dec_03.SM_maus_dec_03" :`3` "/Game/Environment/meshes/mausoleum/SM_maus_dec_04.SM_maus_dec_04" :!type "StaticMesh Object Reference") :!label _label)
        ;;[1 0.7602 0.2323] decor on doubleDoor?
        (if (not (`KismetMathLibrary.BooleanNAND` (== (`local.L_doorType`) 0) (== (`local.L_decorPosition`) 2)))
          ;;[0.1604 0.5721 1] add decor piece
          ;;;[1 1 1] set second decor transform (doubleDoor only)
          (bind _returnvalue_15 (`AddComponent|NODE_AddStaticMeshComponent-15` :`RelativeTransform` (`KismetMathLibrary.MakeTransform` (-28.0 128.0 148.0) (struct) (0.6 1.0 0.6))))
          ;;;[1 1 1] set secondary mesh
          (`StaticMeshComponent.SetStaticMesh` _returnvalue_15 (`local.L_decorMesh`)))
        ;;;[1 1 1] set main decor transform
        (bind _returnvalue_16 (`AddComponent|NODE_AddStaticMeshComponent-17` :`RelativeTransform` (`KismetMathLibrary.MakeTransform` (`KismetMathLibrary.SelectVector` (`KismetMathLibrary.MakeVector` 0.0 175.0 (`KismetMathLibrary.SelectFloat` 290.0 256.0 _l_flatroof_)) (`KismetMathLibrary.MakeVector` (`KismetMathLibrary.SelectFloat` 28.0 0.0 _returnvalue_5) 128.0 148.0) _returnvalue_4) (struct) (`KismetMathLibrary.SelectVector` (`KismetMathLibrary.MakeVector` _returnvalue_2 _returnvalue_2 _returnvalue_2) (`KismetMathLibrary.MakeVector` _returnvalue_8 1.0 _returnvalue_8) _returnvalue_4))))
        ;;;;[0.1604 0.5721 1] set main mesh
        (`StaticMeshComponent.SetStaticMesh` _returnvalue_16 (`local.L_decorMesh`))
        ;;[0.1604 0.5721 1] switch and add second decor mesh
        (`/Engine/EditorBlueprintResources/StandardMacros.DoOnce` false
          (:`Completed`
            ;;;[1 0.7602 0.2323] should add second mesh?
            (if (and (or _returnvalue_6 (== _l_decortype 3)) (`KismetMathLibrary.RandomBool`))
              ;;;[0.2778 0.06791 1] switch decor index
              (set `local.L_decorType` (`KismetMathLibrary.SelectInt` 3 1 _returnvalue_6))
              (goto _label))))))))

(fn `buildStandard`
  (bind (_columnoffset_x _columnoffset_y) (`KismetMathLibrary.BreakVector2D` (`self.columnOffset`)))
  (bind (_columnoffset_x_2 _columnoffset_y_2) (`KismetMathLibrary.BreakVector2D` (`self.columnOffset`)))
  (bind (_crownoffset_x _crownoffset_y) (`KismetMathLibrary.BreakVector2D` (`self.crownOffset`)))
  (bind _decortransform (`self.decorTransform`))
  (bind _windowmesh (`self.windowMesh`))
  (bind _decormesh (`self.decorMesh`))
  (bind _windowtransforms (`self.windowTransforms`))
  (bind _returnvalue (== 0 (`self.doorType`)))
  (`|ExecutionSequence`
    (:`then_0`
      ;[1 1 1] change roof type
      (`StaticMeshComponent.SetStaticMesh` (`self.roof`) (select `bool` (`self.useFlatRoof?`) :`false` "/Game/Environment/meshes/mausoleum/SM_maus_roofAngle.SM_maus_roofAngle" :`true` "/Game/Environment/meshes/mausoleum/SM_maus_roofFlat.SM_maus_roofFlat" :!type "StaticMesh Object Reference")))
    (:`then_1`
      ;[1 1 1] change doorType
      (`StaticMeshComponent.SetStaticMesh` (`self.door`) (select `int` (`self.doorType`) :`0` "/Game/Environment/meshes/mausoleum/SM_maus_door_01.SM_maus_door_01" :`1` "/Game/Environment/meshes/mausoleum/SM_maus_door_02.SM_maus_door_02" :`2` "/Game/Environment/meshes/mausoleum/SM_maus_door_03.SM_maus_door_03" :!type "StaticMesh Object Reference")))
    (:`then_2`
      ;[1 1 1] build doorHandle(s)
      ;;[0.1604 0.5721 1] build baseHandle
      ;;;[1 1 1] position baseHandle
      (bind _returnvalue_2 (`AddComponent|NODE_AddStaticMeshComponent-2` :`RelativeTransform` (`KismetMathLibrary.MakeTransform` (`KismetMathLibrary.MakeVector` (`KismetMathLibrary.SelectFloat` 5.0 -53.0 _returnvalue) 128.0 85.0))))
      ;;;[1 1 1] change handleMesh
      (`StaticMeshComponent.SetStaticMesh` _returnvalue_2 (select `bool` (`self.useFancyHandle?`) :`false` "/Game/Environment/meshes/mausoleum/SM_maus_doorHandle_01.SM_maus_doorHandle_01" :`true` "/Game/Environment/meshes/mausoleum/SM_maus_doorHandle_02.SM_maus_doorHandle_02" :!type "StaticMesh Object Reference"))
      ;;[1 0.7602 0.2323] is doubleDoor?
      (if _returnvalue
        ;;[0.1604 0.5721 1] add secondHandle
        (bind _returnvalue_3 (`AddComponent|NODE_AddStaticMeshComponent-3` :`RelativeTransform` (`KismetMathLibrary.MakeTransform` (-5.0 128.0 85.0) (struct) (-1.0 1.0 1.0))))
        (`StaticMeshComponent.SetStaticMesh` _returnvalue_3 (select `bool` (`self.useFancyHandle?`) :`false` "/Game/Environment/meshes/mausoleum/SM_maus_doorHandle_01.SM_maus_doorHandle_01" :`true` "/Game/Environment/meshes/mausoleum/SM_maus_doorHandle_02.SM_maus_doorHandle_02" :!type "StaticMesh Object Reference"))
        ;;[0.1604 0.5721 1] adjust lock to doubleDoor
        (`SceneComponent.K2_SetRelativeLocation` (`self.lock`) (-5.0 128.0 100.0) false false)))
    (:`then_3`
      ;[1 1 1] build columns
      ;;[1 0.7602 0.2323] are columns enabled?
      (if (> (`self.columnType`) 0)
        ;;[0.1604 0.5721 1] build 1st column
        ;;;[1 1 1] set column location
        (bind _returnvalue_4 (`AddComponent|NODE_AddStaticMeshComponent-4` :`RelativeTransform` (`KismetMathLibrary.MakeTransform` (`KismetMathLibrary.MakeVector` (+ _columnoffset_x_2 94.0) (+ _columnoffset_y_2 159.0)))))
        ;;;[1 1 1] set column meshType
        (`StaticMeshComponent.SetStaticMesh` _returnvalue_4 (select `bool` (== (`self.columnType`) 2) :`false` "/Game/Environment/meshes/mausoleum/SM_maus_col_01.SM_maus_col_01" :`true` "/Game/Environment/meshes/mausoleum/SM_maus_col_02.SM_maus_col_02" :!type "StaticMesh Object Reference"))
        ;;[0.1604 0.5721 1] build 2nd column
        ;;;[1 1 1] set column location
        (bind _returnvalue_5 (`AddComponent|NODE_AddStaticMeshComponent-5` :`RelativeTransform` (`KismetMathLibrary.MakeTransform` (`KismetMathLibrary.MakeVector` (- -94.0 _columnoffset_x) (+ _columnoffset_y 159.0)))))
        ;;;[1 1 1] set column meshType
        (`StaticMeshComponent.SetStaticMesh` _returnvalue_5 (select `bool` (== (`self.columnType`) 2) :`false` "/Game/Environment/meshes/mausoleum/SM_maus_col_01.SM_maus_col_01" :`true` "/Game/Environment/meshes/mausoleum/SM_maus_col_02.SM_maus_col_02" :!type "StaticMesh Object Reference"))))
    (:`then_4`
      ;[1 1 1] build crown
      ;;[1 0.7602 0.2323] is crown enabled?
      (if (> (`self.crownType`) 0)
        ;;[0.1604 0.5721 1] set location/scale
        (bind _returnvalue_6 (`AddComponent|NODE_AddStaticMeshComponent-6` :`RelativeTransform` (`KismetMathLibrary.MakeTransform` (`KismetMathLibrary.MakeVector` 0.0 (+ _crownoffset_x 165.0) (+ _crownoffset_y 290.0)) (struct) (`self.crownScale`))))
        ;;[0.1604 0.5721 1] change mesh type
        (`StaticMeshComponent.SetStaticMesh` _returnvalue_6 (select `int` (- (`self.crownType`) 1) :`0` "/Game/Environment/meshes/mausoleum/SM_maus_cap_01.SM_maus_cap_01" :`1` "/Game/Environment/meshes/mausoleum/SM_maus_cap_02.SM_maus_cap_02" :`2` "/Game/Environment/meshes/mausoleum/SM_maus_cap_03.SM_maus_cap_03" :!type "StaticMesh Object Reference"))))
    (:`then_5`
      ;[1 1 1] build windows
      ;;[1 0.7602 0.2323] are windows enabled?
      (if (`KismetArrayLibrary.Array_IsValidIndex` _windowmesh)
        (for (_ _array_index) _windowmesh
          ;;[0.1604 0.5721 1] add single window
          ;;;[1 1 1] set mesh transform
          (bind _returnvalue_7 (`AddComponent|NODE_AddStaticMeshComponent-7` :`RelativeTransform` (`KismetMathLibrary.SelectTransform` (`|GetArrayItem` _windowtransforms _array_index) (`KismetMathLibrary.MakeTransform` (0.0 0.0 0.0)) (`KismetArrayLibrary.Array_IsValidIndex` _windowtransforms _array_index))))
          ;;;[1 1 1] set mesh type
          (`StaticMeshComponent.SetStaticMesh` _returnvalue_7 (`|GetArrayItem` (`self.windowMesh`) _array_index)))))
    (:`then_6`
      ;[1 1 1] build decor
      ;;[1 0.7602 0.2323] is decor enabled?
      (if (`KismetArrayLibrary.Array_IsValidIndex` _decormesh)
        (for (_ _array_index_2) _decormesh
          ;;[0.1604 0.5721 1] add single decor piece
          ;;;[1 1 1] set mesh transform
          (bind _returnvalue_8 (`AddComponent|NODE_AddStaticMeshComponent-8` :`RelativeTransform` (`KismetMathLibrary.SelectTransform` (`|GetArrayItem` _decortransform _array_index_2) (`KismetMathLibrary.MakeTransform` (0.0 0.0 0.0)) (`KismetArrayLibrary.Array_IsValidIndex` _decortransform _array_index_2))))
          ;;;[1 1 1] set mesh type
          (`StaticMeshComponent.SetStaticMesh` _returnvalue_8 (`|GetArrayItem` (`self.decorMesh`) _array_index_2)))))))

(fn `UserConstructionScript`
  ;[1 0.7602 0.2323] randomize mausoleum
  (if (`self.randomize`)
    (`self.buildRandom`)
    (else
      (`self.buildStandard`))))