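; Spline-driven fence builder that assembles fence sections, posts and gates entirely in the construction script.
; It splits the spline, whole or per segment, into fitted sections of spline meshes, using shorter mesh variants for partial lengths.
; Gate distances cut gaps sized by stepping to a straight-line width, optionally filled with rotated gate meshes.
; AddCap places posts by cap mode, stagger and gate edges; collision is optionally applied last.
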(fn `addCap`
  (params (Distance :type "Float (single-precision)") (`gateStart/End` :type Integer) (`splineStart/End` :type Integer))
  (returns (staticMeshComponent :type "StaticMeshComponent Object Reference"))
  (bind _returnvalue (== `splineStart/End` 1))
  (bind _spline (`self.Spline`))
  (bind _returnvalue_2 (* (.x (`.BoxExtent` (`KismetMathLibrary.BreakBoxSphereBounds` (`StaticMesh.GetBounds` (`self.capMesh`))))) 0.85))
  (bind _returnvalue_3 (`KismetMathLibrary.SelectFloat` _returnvalue_2 (`self.offsetAmount`) (> `gateStart/End` 0)))
  (bind _returnvalue_4 (`KismetMathLibrary.SelectFloat` Distance (`KismetMathLibrary.SelectFloat` (- Distance _returnvalue_3) (+ Distance _returnvalue_3) (== `gateStart/End` 2)) (or (not (`self.offsetColumns?`)) (and (not (`self.closeLoop`)) _returnvalue))))
  (bind _returnvalue_5 (`SplineComponent.GetLocationAtDistanceAlongSpline` _spline _returnvalue_4 "Local"))
  (bind _returnvalue_6 (`SplineComponent.GetRotationAtDistanceAlongSpline` _spline _returnvalue_4 "Local"))
  ;[1 1 1] Create initial column
  (bind _returnvalue_7 (`AddComponent|NODE_AddStaticMeshComponent-0` :`RelativeTransform` (`KismetMathLibrary.MakeTransform` _returnvalue_5 (`KismetMathLibrary.SelectRotator` (`KismetMathLibrary.MakeRotator` (.roll _returnvalue_6) (.pitch _returnvalue_6) (+ (.yaw _returnvalue_6) 180.0)) _returnvalue_6 _returnvalue) (`self.capScale`))))
  (`StaticMeshComponent.SetStaticMesh` _returnvalue_7 (`self.capMesh`))
  (if (not (or (`self.closeLoop`) (not (`self.offsetColumns?`)) (== `splineStart/End` 0)))
    (`SceneComponent.K2_SetRelativeLocation` _returnvalue_7 (+ _returnvalue_5 (* (`SceneComponent.GetForwardVector` _returnvalue_7) _returnvalue_2)) false false))
  (return _returnvalue_7))

(fn `UserConstructionScript`
  (bind _returnvalue_x (`KismetMathLibrary.BreakVector` (`self.GetActorScale3D`)))
  (bind _spline (`self.Spline`))
  (bind _startdistance (`self.startDistance`))
  (bind _fencescale_x (`KismetMathLibrary.BreakVector` (`self.fenceScale`)))
  (bind _gatescale_x (`KismetMathLibrary.BreakVector` (`self.gateScale`)))
  (bind (_fencescale_x_2 _fencescale_y _fencescale_z) (`KismetMathLibrary.BreakVector` (`self.fenceScale`)))
  (bind _fencemesh (`self.fenceMesh`))
  (bind _sectioncurrentindex (`self.sectionCurrentIndex`))
  (bind _gateendcap (`self.gateEndCap`))
  (bind _gate_gapalwayscapped_ (`self.gate/GapAlwaysCapped?`))
  (bind _setgateends (`self.setGateEnds`))
  (bind _independentsegments_ (`self.independentSegments?`))
  (bind _gate_gaplocations (`self.gate/GapLocations`))
  (bind _startdistance_2 (`self.startDistance`))
  (bind _testdistances (`self.testDistances`))
  (bind _enddistance (`self.endDistance`))
  (bind _spline_2 (`self.Spline`))
  (bind _gatecurrentdistance (`self.gateCurrentDistance`))
  (bind _spline_3 (`self.Spline`))
  (bind _sectioncurrentindex_2 (`self.sectionCurrentIndex`))
  (bind _gaterotations (`self.gateRotations`))
  (bind _captype (`self.capType`))
  (bind _spline_4 (`self.Spline`))
  (bind _spline_5 (`self.Spline`))
  (bind _currentstartdistance (`self.currentStartDistance`))
  (bind _currentenddistance (`self.currentEndDistance`))
  (bind _sectioncount (`self.sectionCount`))
  (bind _gatestartlocation (`self.gateStartLocation`))
  (bind _sectionlength (`self.sectionLength`))
  (bind _spline_segmentlength (`self.spline/segmentLength`))
  (bind _tangentclamp (`self.tangentClamp`))
  (bind _testdistances_2 (`self.testDistances`))
  (bind _testdistances_3 (`self.testDistances`))
  (bind _returnvalue (`KismetArrayLibrary.Array_IsValidIndex` _gate_gaplocations))
  (bind _returnvalue_2 (`KismetArrayLibrary.Array_Find` (`self.gate/GapLocations`) (`self.gateStartDistance`)))
  (bind _returnvalue_3 (`SplineComponent.GetNumberOfSplinePoints` (`self.Spline`)))
  (bind _returnvalue_4 (/ (`self.spline/segmentLength`) (`self.originLength`)))
  (bind _returnvalue_5 (> (`self.fittingType`) 1))
  (bind _returnvalue_6 (== (`self.sectionCurrentIndex`) 0))
  (bind _returnvalue_7 (* _sectioncurrentindex_2 _sectionlength))
  (bind _returnvalue_8 (`KismetMathLibrary.ClampVectorSize` (`SplineComponent.GetTangentAtDistanceAlongSpline` _spline _currentstartdistance "Local") 0.0 _tangentclamp))
  (bind _returnvalue_9 (`KismetMathLibrary.FTrunc` _returnvalue_4))
  (bind _roll (.roll (`KismetMathLibrary.FindLookAtRotation` _gatestartlocation (`self.gateEndLocation`))))
  (bind _pitch (.pitch (`KismetMathLibrary.FindLookAtRotation` _gatestartlocation (`self.gateEndLocation`))))
  (bind _yaw (.yaw (`KismetMathLibrary.FindLookAtRotation` _gatestartlocation (`self.gateEndLocation`))))
  (bind _returnvalue_10 (* (+ _sectioncurrentindex_2 1) _sectionlength))
  (bind _returnvalue_11 (- (`SplineComponent.GetNumberOfSplinePoints` _spline_4) 1))
  (bind _returnvalue_12 (/ (- (`self.currentEndDistance`) (`self.currentStartDistance`)) (`self.originLength`)))
  (bind _returnvalue_13 (+ _startdistance_2 _returnvalue_10))
  (bind _returnvalue_14 (== (`KismetMathLibrary.FMod` (`KismetMathLibrary.Conv_IntToDouble` _sectioncurrentindex) (`KismetMathLibrary.Conv_IntToDouble` (`self.capStaggerAmount`))) 0.0))
  (`|ExecutionSequence`
    (:`then_0`
      ;[1 1 1] Set Mesh Length
      (set `self.originLength` (* _fencescale_x 2.0 (.x (`.BoxExtent` (`KismetMathLibrary.BreakBoxSphereBounds` (`StaticMesh.GetBounds` (`|GetArrayItem` (`self.fenceMesh`)))))) _returnvalue_x))
      (set `self.gateSize` (`KismetMathLibrary.SelectFloat` (`self.gapSize`) (* _gatescale_x 2.0 (.x (`.BoxExtent` (`KismetMathLibrary.BreakBoxSphereBounds` (`StaticMesh.GetBounds` (`self.gateMesh`))))) _returnvalue_x) (`self.gapOnly?`)))
      ;[1 1 1] Should look for Gates?/Set Gates index
      (set `self.hasGates` _returnvalue)
      (set `self.testDistances` (select `bool` _returnvalue :`false` (`|MakeArray`) :`true` _gate_gaplocations))
      ;[1 1 1] Close Loop (custom)
      (`SplineComponent.SetClosedLoop` (`self.Spline`) (`self.closeLoop`) true)
      (`|ExecutionSequence`
        (:`then_0`
          ;[1 1 1] Run for each Segment independently
          (if (`self.independentSegments?`)
            ;[1 1 1] Set/Run Segment Loop
            (bind _output_get (set `self.segmentEndIndex` (`KismetMathLibrary.SelectInt` (- _returnvalue_3 1) (- _returnvalue_3 2) (`self.closeLoop`))))
            (for _index (range (+ _output_get 1))
              ;[1 1 1] Set Start/End Distance and Current Index
              (bind _output_get_2 (set `self.segmentCurrentIndex` _index))
              (set `self.startDistance` (`SplineComponent.GetDistanceAlongSplineAtSplinePoint` _spline_3 _output_get_2))
              (bind _returnvalue_15 (+ _output_get_2 1))
              (set `self.endDistance` (`SplineComponent.GetDistanceAlongSplineAtSplinePoint` _spline_3 _returnvalue_15))
              ;[1 0.7602 0.2323] Fix final section warping (linear-independent segment only)
              (set `self.linearCorners` (and (`|EnumEquality` (`SplineComponent.GetSplinePointType` _spline_2 _returnvalue_15) "Linear") (`|EnumEquality` (`SplineComponent.GetSplinePointType` _spline_2 (`self.segmentCurrentIndex`)) "Linear")))
              ;[1 1 1] Add Cap per Segment (if Independent)
              (if (== (`self.capType`) 3)
                (`|ExecutionSequence`
                  (:`then_0`
                    ;[1 0.7602 0.2323] Is Cap Blocked by Gate?
                    (for _array_element (`self.gateOccupiedArea`)
                      (if (`KismetMathLibrary.InRange_FloatFloat` _startdistance (`KismetMathLibrary.BreakVector2D` _array_element) (`.Y` (`KismetMathLibrary.BreakVector2D` _array_element)))
                        (set `self.capBlocked` true)
                        (break))))
                  (:`then_1`
                    (if (`self.capBlocked`)
                      (set `self.capBlocked` false)
                      (else
                        (`self.addCap` _startdistance 0 (`KismetMathLibrary.SelectInt` 1 0 (== (`self.segmentCurrentIndex`) 0)))))
                    ;[1 1 1] Set Spline/Segment Length
                    (set `self.spline/segmentLength` (`KismetMathLibrary.SelectFloat` (- (`self.endDistance`) (`self.startDistance`)) (`SplineComponent.GetSplineLength` (`self.Spline`)) (`self.independentSegments?`)) :!label _label)
                    ;[1 1 1] Set Section Count
                    (set `self.sectionCount` (select `int` (`self.fittingType`) :`0` (- _returnvalue_9 1) :`1` _returnvalue_9 :`2` (`KismetMathLibrary.FCeil` _returnvalue_4) :`3` _returnvalue_9))
                    ;[1 1 1] Set Section Length
                    (set `self.sectionLength` (`KismetMathLibrary.SelectFloat` (/ (`self.spline/segmentLength`) (`self.sectionCount`)) (`self.originLength`) _returnvalue_5))
                    ;[1 1 1] Set Loop Count/Run Loop
                    (bind _output_get_3 (set `self.sectionEndIndex` (`KismetMathLibrary.SelectInt` (- _sectioncount 1) _sectioncount _returnvalue_5)))
                    (for _index_2 (range (+ _output_get_3 1))
                      ;[1 1 1] set Section Index and Start/End Distances
                      (set `self.sectionCurrentIndex` _index_2)
                      (set `self.currentEndDistance` (`KismetMathLibrary.SelectFloat` (`KismetMathLibrary.SelectFloat` _enddistance _returnvalue_13 (> _returnvalue_13 _enddistance)) (`KismetMathLibrary.SelectFloat` _spline_segmentlength _returnvalue_10 (> _returnvalue_10 _spline_segmentlength)) (`self.independentSegments?`)))
                      (if (`self.setGateEnds`)
                        ;;[0.1604 0.5721 1] Adjust Next Section to Fit Gate
                        (if (not (> (`self.gateEndDistance`) (`self.currentEndDistance`)))
                          (set `self.gateEndCap` true)
                          (set `self.currentStartDistance` (`self.gateEndDistance`))
                          (set `self.setGateEnds` false)
                          (`|ExecutionSequence` :!label _label_2
                            (:`then_0`
                              ;[1 1 1] Is Gate/Gap Section?
                              (if (`self.hasGates`)
                                (for (_array_element_2 _array_index) _testdistances_2
                                  ;;[1 0.7602 0.2323] Is Gate Valid?
                                  (if (> (+ (`self.gateSize`) _array_element_2) (`SplineComponent.GetSplineLength` (`self.Spline`)))
                                    (`KismetArrayLibrary.Array_Remove` _testdistances_2 _array_index)
                                    (else
                                      ;;[0.1604 0.5721 1] Is Current Section at Gate?
                                      (if (> (`self.currentEndDistance`) _array_element_2)
                                        ;;[0.1604 0.5721 1] Set Gate Starting Parameters
                                        (bind _output_get_4 (set `self.gateCurrentDistance` _array_element_2))
                                        (set `self.gateStartDistance` _output_get_4)
                                        (set `self.setGateEnds` true)
                                        ;;[0.1604 0.5721 1] Remove Entry from Array
                                        (`KismetArrayLibrary.Array_Remove` _testdistances _array_index)
                                        (set `self.hasGates` (`KismetArrayLibrary.Array_IsValidIndex` _testdistances))
                                        (break)))))))
                            (:`then_1`
                              (if (`self.setGateEnds`)
                                ;[1 1 1] Set Gate Start
                                (set `self.currentEndDistance` _gatecurrentdistance)
                                (set `self.gateStartLocation` (`SplineComponent.GetLocationAtDistanceAlongSpline` (`self.Spline`) _gatecurrentdistance "Local"))
                                (set `self.gateTestAmount` (`KismetMathLibrary.FTrunc` (/ (- (`SplineComponent.GetSplineLength` (`self.Spline`)) (`self.gateCurrentDistance`)) (`self.gateTestDistance`))))
                                (`|ExecutionSequence`
                                  (:`then_0`
                                    ;[1 1 1] Find Gate Location
                                    ;;[0.1604 0.5721 1] Set Loop Counter/Run Loop
                                    (for _ (range (+ (`self.gateTestAmount`) 1))
                                      (`|ExecutionSequence`
                                        (:`then_0`
                                          ;;[0.1604 0.5721 1] First Run Set Gate End Minimum
                                          (`/Engine/EditorBlueprintResources/StandardMacros.DoOnce` false :!label _label_3
                                            (:`Completed`
                                              (bind _output_get_5 (set `self.gateCurrentDistance` (+ (`self.gateCurrentDistance`) (`self.gateSize`))))
                                              (set `self.gateEndDistance` _output_get_5))))
                                        (:`then_1`
                                          ;;[0.1604 0.5721 1] Find Gate End Location/Distance
                                          ;;;[1 1 1] Increment Test Distance
                                          (bind _output_get_6 (set `self.gateCurrentDistance` (+ (`self.gateCurrentDistance`) (`self.gateTestDistance`))))
                                          (bind _returnvalue_16 (`SplineComponent.GetLocationAtDistanceAlongSpline` (`self.Spline`) _output_get_6 "Local"))
                                          ;;;[1 1 1] Test Start-End Length
                                          (if (> (`KismetMathLibrary.Vector_Distance` _returnvalue_16 (`self.gateStartLocation`)) (`self.gateSize`))
                                            ;;;[1 1 1] Set Gate End
                                            (set `self.gateEndLocation` _returnvalue_16)
                                            (set `self.gateEndDistance` (`self.gateCurrentDistance`))
                                            (break))))))
                                  (:`then_1`
                                    (goto _label_3 :!via `Reset`))
                                  (:`then_2`
                                    ;;[1 0.7602 0.2323] Add Gate Bounds to Clear
                                    (`KismetArrayLibrary.Array_Add` (`self.gateOccupiedArea`) (`KismetMathLibrary.MakeVector2D` (`self.gateStartDistance`) (`self.gateEndDistance`)))
                                    (if (`self.hasGates`)
                                      ;;[1 0.7602 0.2323] Clear overlapping Gates
                                      (for (_array_element_3 _array_index_2) _testdistances_3
                                        (for _array_element_4 (`self.gateOccupiedArea`)
                                          (if (`KismetMathLibrary.InRange_FloatFloat` _array_element_3 (`KismetMathLibrary.BreakVector2D` _array_element_4) (`.Y` (`KismetMathLibrary.BreakVector2D` _array_element_4)))
                                            (`KismetArrayLibrary.Array_Remove` _testdistances_3 _array_index_2)
                                            (break)))))
                                    ;[1 1 1] Add Gate Mesh
                                    (if (not (`self.gapOnly?`))
                                      (bind _returnvalue_17 (`AddComponent|NODE_AddStaticMeshComponent-10` :`RelativeTransform` (`KismetMathLibrary.MakeTransform` (0.0 0.0 0.0) (struct) (`self.gateScale`))))
                                      (`StaticMeshComponent.SetStaticMesh` _returnvalue_17 (`self.gateMesh`))
                                      (`SceneComponent.K2_SetRelativeLocation` _returnvalue_17 _gatestartlocation false false)
                                      (if (`KismetArrayLibrary.Array_IsValidIndex` _gaterotations _returnvalue_2)
                                        (`SceneComponent.K2_SetRelativeRotation` _returnvalue_17 (`KismetMathLibrary.MakeRotator` _roll _pitch (+ _yaw (`|GetArrayItem` _gaterotations _returnvalue_2))) false false)
                                        (else
                                          (`SceneComponent.K2_SetRelativeRotation` _returnvalue_17 (`KismetMathLibrary.MakeRotator` _roll _pitch _yaw) false false))))))))
                            (:`then_2`
                              ;[1 1 1] Add columns per fence section (w/ gates)
                              (if (== (`self.capType`) 2)
                                ;;[1 0.7602 0.2323] cap can be placed according to stagger rule (or is gate end/first section)
                                (if (== _sectioncurrentindex 0)
                                  ;;[0.1604 0.5721 1] Add section cap
                                  (`self.addCap` (`self.currentStartDistance`) (`KismetMathLibrary.SelectInt` 2 0 _gateendcap) (`KismetMathLibrary.SelectInt` 1 0 (or (and (== (`self.segmentCurrentIndex`) 0) _independentsegments_ _returnvalue_6) (and _returnvalue_6 (not _independentsegments_)))) :!label _label_4)
                                  (set `self.gateEndCap` false)
                                  (if (and _setgateends (== (`self.capStaggerAmount`) 1))
                                    _)
                                  (elif (or _returnvalue_14 (and _gateendcap _gate_gapalwayscapped_))
                                    (goto _label_4)
                                    (else
                                      ;;[0.1604 0.5721 1] Add Cap to Gate Start (allSections only)
                                      (if (and _setgateends _gate_gapalwayscapped_)
                                        (`self.addCap` (`self.currentEndDistance`) 1)))))
                                (else
                                  ;[1 1 1] Add Gaps to Gate (if Override Enabled)
                                  (if (and (`self.gate/GapAlwaysCapped?`) (`self.setGateEnds`))
                                    (`self.addCap` (`self.gateStartDistance`) 1)
                                    (if (not _returnvalue_14)
                                      (`self.addCap` (`self.gateEndDistance`) 2))))))
                            (:`then_3`
                              ;[1 1 1] Create Fence Section
                              (bind _returnvalue_18 (`AddComponent|NODE_AddSplineMeshComponent-0`))
                              (`SplineMeshComponent.SetStartScale` _returnvalue_18 (`KismetMathLibrary.MakeVector2D` _fencescale_y _fencescale_z) true)
                              (`SplineMeshComponent.SetEndScale` _returnvalue_18 (`KismetMathLibrary.MakeVector2D` _fencescale_y _fencescale_z) true)
                              ;[1 1 1] assign mesh variant based on section size (full, 3/4, 1/2, 1/4)
                              (if (or (> _returnvalue_12 0.75) (not (`KismetArrayLibrary.Array_IsValidIndex` _fencemesh 1)))
                                (`StaticMeshComponent.SetStaticMesh` _returnvalue_18 (`|GetArrayItem` _fencemesh))
                                (set `self.tangentClamp` (`self.sectionLength`))
                                (elif (or (> _returnvalue_12 0.5) (not (`KismetArrayLibrary.Array_IsValidIndex` _fencemesh 2)))
                                  (`StaticMeshComponent.SetStaticMesh` _returnvalue_18 (`|GetArrayItem` _fencemesh 1))
                                  (set `self.tangentClamp` (* 0.75 (`self.sectionLength`)))
                                  (elif (or (> _returnvalue_12 0.25) (not (`KismetArrayLibrary.Array_IsValidIndex` _fencemesh 3)))
                                    (`StaticMeshComponent.SetStaticMesh` _returnvalue_18 (`|GetArrayItem` _fencemesh 2))
                                    (set `self.tangentClamp` (* 0.5 (`self.sectionLength`)))
                                    (else
                                      (`StaticMeshComponent.SetStaticMesh` _returnvalue_18 (`|GetArrayItem` _fencemesh 3))
                                      (set `self.tangentClamp` (* 0.25 (`self.sectionLength`)))))))
                              ;[1 1 1] Set Section Start/End points
                              (`SplineMeshComponent.SetStartAndEnd` _returnvalue_18 (`SplineComponent.GetLocationAtDistanceAlongSpline` _spline _currentstartdistance "Local") _returnvalue_8 (`SplineComponent.GetLocationAtDistanceAlongSpline` _spline _currentenddistance "Local") (`KismetMathLibrary.SelectVector` _returnvalue_8 (`KismetMathLibrary.ClampVectorSize` (`SplineComponent.GetTangentAtDistanceAlongSpline` _spline _currentenddistance "Local") 0.0 _tangentclamp) (and (== (`self.sectionCurrentIndex`) (`self.sectionEndIndex`)) (`self.linearCorners`))) true))))
                        (else
                          (set `self.currentStartDistance` (`KismetMathLibrary.SelectFloat` (+ _startdistance_2 _returnvalue_7) _returnvalue_7 (`self.independentSegments?`)))
                          (goto _label_2))))))
                (else
                  (goto _label))))
            (else
              (goto _label))))
        (:`then_1`
          ;[1 1 1] Add Cap per Segment (non Independent)
          (if (and (not (`self.independentSegments?`)) (== (`self.capType`) 3))
            (for _index_3 (range (+ _returnvalue_11 1))
              (`|ExecutionSequence`
                (:`then_0`
                  ;[1 0.7602 0.2323] Is Cap Blocked by Gate?
                  (for _array_element_5 (`self.gateOccupiedArea`)
                    (bind _returnvalue_19 (`SplineComponent.GetDistanceAlongSplineAtSplinePoint` _spline_4 _index_3))
                    (if (`KismetMathLibrary.InRange_FloatFloat` _returnvalue_19 (`KismetMathLibrary.BreakVector2D` _array_element_5) (`.Y` (`KismetMathLibrary.BreakVector2D` _array_element_5)))
                      (set `self.capBlocked` true)
                      (break))))
                (:`then_1`
                  (if (`self.capBlocked`)
                    (set `self.capBlocked` false)
                    (else
                      (`self.addCap` _returnvalue_19 0 (`KismetMathLibrary.SelectInt` 1 (`KismetMathLibrary.SelectInt` 2 0 (== _index_3 _returnvalue_11)) (== _index_3 0))))))))))
        (:`then_2`
          ;[1 1 1] Add Start/End Caps
          (if (and (not (`self.closeLoop`)) (> _captype 0))
            ;;[0.1604 0.5721 1] Add Cap at Start of Spline (Start/End only)
            (if (== _captype 1)
              (`self.addCap` (`SplineComponent.GetDistanceAlongSplineAtSplinePoint` _spline_5 0) 0 1)
              ;;[0.1604 0.5721 1] Add Cap at End of Spline
              (`self.addCap` (`SplineComponent.GetDistanceAlongSplineAtSplinePoint` _spline_5 (- (`SplineComponent.GetNumberOfSplinePoints` _spline_5) 1)) 0 2 :!label _label_5)
              (elif (or (and (== _captype 3) (`self.independentSegments?`)) (== _captype 2))
                (goto _label_5)))))))
    (:`then_1`
      ;[1 1 1] Add Collision to Spline Meshes (bogs-down engine if editing while collision is enabled)
      (if (`self.enableCollision?`)
        (for _array_element_6 (`SceneComponent.GetChildrenComponents` (`self.DefaultSceneRoot`) false)
          (if (== (`GameplayStatics.GetObjectClass` _array_element_6) "/Script/Engine.SplineMeshComponent")
            (`PrimitiveComponent.SetCollisionEnabled` (cast `SplineMeshComponent` _array_element_6 :!pure true) (`self.collisionType`))))))))