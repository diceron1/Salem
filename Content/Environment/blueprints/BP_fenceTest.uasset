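; Spline-driven fence builder that lays fence meshes, gates or gaps, and caps along an editable spline in the construction script.
; Sections follow a fitting mode and run over the whole spline or per segment, with tangent adjustment against warping at linear corners.
; Gates at listed distances step along the curve to find their straight-line end, trimming adjacent sections.
; Caps follow a placement mode, with per-point caps skipped inside gate spans.
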(fn `addCap`
  (params (Distance :type "Float (single-precision)"))
  (returns (staticMeshComponent :type "StaticMeshComponent Object Reference"))
  (bind _spline (`self.Spline`))
  (bind _returnvalue (`AddComponent|NODE_AddStaticMeshComponent-0` :`RelativeTransform` (`KismetMathLibrary.MakeTransform` (0.0 0.0 0.0) (struct) (`self.capScale`))))
  (`StaticMeshComponent.SetStaticMesh` _returnvalue (`self.capMesh`))
  (`SceneComponent.K2_SetRelativeLocationAndRotation` _returnvalue (`SplineComponent.GetLocationAtDistanceAlongSpline` _spline Distance "Local") (`SplineComponent.GetRotationAtDistanceAlongSpline` _spline Distance "Local") false false)
  (return _returnvalue))

(fn `UserConstructionScript`
  (bind _returnvalue_x (`KismetMathLibrary.BreakVector` (`self.GetActorScale3D`)))
  (bind _spline (`self.Spline`))
  (bind _sectionlength (`self.sectionLength`))
  (bind _startdistance (`self.startDistance`))
  (bind _fencescale_x (`KismetMathLibrary.BreakVector` (`self.fenceScale`)))
  (bind _gatescale_x (`KismetMathLibrary.BreakVector` (`self.gateScale`)))
  (bind (_fencescale_x_2 _fencescale_y _fencescale_z) (`KismetMathLibrary.BreakVector` (`self.fenceScale`)))
  (bind _gate_gapdistances (`self.gate/GapDistances`))
  (bind _startdistance_2 (`self.startDistance`))
  (bind _testdistances (`self.testDistances`))
  (bind _enddistance (`self.endDistance`))
  (bind _spline_2 (`self.Spline`))
  (bind _gatecurrentdistance (`self.gateCurrentDistance`))
  (bind _spline_3 (`self.Spline`))
  (bind _sectioncurrentindex (`self.sectionCurrentIndex`))
  (bind _currentstartdistance (`self.currentStartDistance`))
  (bind _currentenddistance (`self.currentEndDistance`))
  (bind _gaterotations (`self.gateRotations`))
  (bind _captype (`self.capType`))
  (bind _spline_4 (`self.Spline`))
  (bind _spline_5 (`self.Spline`))
  (bind _sectioncount (`self.sectionCount`))
  (bind _gatestartlocation (`self.gateStartLocation`))
  (bind _sectionlength_2 (`self.sectionLength`))
  (bind _testdistances_2 (`self.testDistances`))
  (bind _testdistances_3 (`self.testDistances`))
  (bind _returnvalue (`KismetArrayLibrary.Array_IsValidIndex` _gate_gapdistances))
  (bind _returnvalue_2 (`KismetArrayLibrary.Array_Find` (`self.gate/GapDistances`) (`self.gateStartDistance`)))
  (bind _returnvalue_3 (`SplineComponent.GetNumberOfSplinePoints` (`self.Spline`)))
  (bind _returnvalue_4 (/ (`self.spline/segmentLength`) (`self.originLength`)))
  (bind _returnvalue_5 (> (`self.fittingType`) 1))
  (bind _returnvalue_6 (* _sectioncurrentindex _sectionlength_2))
  (bind _returnvalue_7 (`KismetMathLibrary.ClampVectorSize` (`SplineComponent.GetTangentAtDistanceAlongSpline` _spline _currentstartdistance "Local") _sectionlength _sectionlength))
  (bind _returnvalue_8 (`KismetMathLibrary.FTrunc` _returnvalue_4))
  (bind _returnvalue_9 (* (+ _sectioncurrentindex 1) _sectionlength_2))
  (bind _returnvalue_10 (+ _startdistance_2 _returnvalue_9))
  ;[1 1 1] Set Mesh Length
  (set `self.originLength` (* _fencescale_x 2.0 (.x (`.BoxExtent` (`KismetMathLibrary.BreakBoxSphereBounds` (`StaticMesh.GetBounds` (`self.fenceMesh`))))) _returnvalue_x))
  (set `self.gateSize` (`KismetMathLibrary.SelectFloat` (`self.gapSize`) (* _gatescale_x 2.0 (.x (`.BoxExtent` (`KismetMathLibrary.BreakBoxSphereBounds` (`StaticMesh.GetBounds` (`self.gateMesh`))))) _returnvalue_x) (`self.gapOnly?`)))
  ;[1 1 1] Should look for Gates?/Set Gates index
  (set `self.hasGates` _returnvalue)
  (set `self.testDistances` (select `bool` _returnvalue :`false` (`|MakeArray`) :`true` _gate_gapdistances))
  ;[1 1 1] Close Loop (custom)
  (`SplineComponent.SetClosedLoop` (`self.Spline`) (`self.closeLoop`) true)
  (`|ExecutionSequence`
    (:`then_0`
      ;[1 1 1] Run for each Segment independently
      (if (`self.independentSegments?`)
        ;[1 1 1] Set/Run Segment Loop
        (bind _output_get (set `self.segmentEndIndex` (`KismetMathLibrary.SelectInt` (- _returnvalue_3 1) (- _returnvalue_3 2) (`self.closeLoop`))))
        (for _index (range (+ _output_get 1))
          ;[1 1 1] Set Start/End Distance and Current Index
          (bind _output_get_2 (set `self.segmentCurrentIndex` _index))
          (set `self.startDistance` (`SplineComponent.GetDistanceAlongSplineAtSplinePoint` _spline_3 _output_get_2))
          (bind _returnvalue_11 (+ _output_get_2 1))
          (set `self.endDistance` (`SplineComponent.GetDistanceAlongSplineAtSplinePoint` _spline_3 _returnvalue_11))
          ;[1 0.7602 0.2323] Fix final section warping (linear-independent segment only)
          (set `self.linearCorners` (and (`|EnumEquality` (`SplineComponent.GetSplinePointType` _spline_2 _returnvalue_11) "Linear") (`|EnumEquality` (`SplineComponent.GetSplinePointType` _spline_2 (`self.segmentCurrentIndex`)) "Linear")))
          ;[1 1 1] Add Cap per Segment (if Independent)
          (if (== (`self.capType`) 3)
            (`|ExecutionSequence`
              (:`then_0`
                ;[1 0.7602 0.2323] Is Cap Blocked by Gate?
                (for _array_element (`self.gateOccupiedArea`)
                  (if (`KismetMathLibrary.InRange_FloatFloat` _startdistance (`KismetMathLibrary.BreakVector2D` _array_element) (`.Y` (`KismetMathLibrary.BreakVector2D` _array_element)))
                    (set `self.capBlocked` true)
                    (break))))
              (:`then_1`
                (if (`self.capBlocked`)
                  (set `self.capBlocked` false)
                  (else
                    (`self.addCap` _startdistance)))
                ;[1 1 1] Set Spline/Segment Length
                (set `self.spline/segmentLength` (`KismetMathLibrary.SelectFloat` (- (`self.endDistance`) (`self.startDistance`)) (`SplineComponent.GetSplineLength` (`self.Spline`)) (`self.independentSegments?`)) :!label _label)
                ;[1 1 1] Set Section Count
                (set `self.sectionCount` (select `int` (`self.fittingType`) :`0` (- _returnvalue_8 1) :`1` _returnvalue_8 :`2` (`KismetMathLibrary.FCeil` _returnvalue_4) :`3` _returnvalue_8))
                ;[1 1 1] Set Section Length
                (set `self.sectionLength` (`KismetMathLibrary.SelectFloat` (/ (`self.spline/segmentLength`) (`self.sectionCount`)) (`self.originLength`) _returnvalue_5))
                ;[1 1 1] Set Loop Count/Run Loop
                (bind _output_get_3 (set `self.sectionEndIndex` (`KismetMathLibrary.SelectInt` (- _sectioncount 1) _sectioncount _returnvalue_5)))
                (for _index_2 (range (+ _output_get_3 1))
                  ;[1 1 1] set Section Index and Start/End Distances
                  (set `self.sectionCurrentIndex` _index_2)
                  (set `self.currentEndDistance` (`KismetMathLibrary.SelectFloat` (`KismetMathLibrary.SelectFloat` _enddistance _returnvalue_10 (> _returnvalue_10 _enddistance)) _returnvalue_9 (`self.independentSegments?`)))
                  (if (`self.setGateEnds`)
                    ;;[0.1604 0.5721 1] Adjust Next Section to Fit Gate
                    (if (not (> (`self.gateEndDistance`) (`self.currentEndDistance`)))
                      (set `self.currentStartDistance` (`self.gateEndDistance`))
                      (set `self.setGateEnds` false)
                      (`|ExecutionSequence` :!label _label_2
                        (:`then_0`
                          ;[1 1 1] Is Gate/Gap Section?
                          (if (`self.hasGates`)
                            (for (_array_element_2 _array_index) _testdistances_2
                              ;;[1 0.7602 0.2323] Is Gate Valid?
                              (if (> (+ (`self.gateSize`) _array_element_2) (`SplineComponent.GetSplineLength` (`self.Spline`)))
                                (`KismetArrayLibrary.Array_Remove` _testdistances_2 _array_index)
                                (else
                                  ;;[0.1604 0.5721 1] Is Current Section at Gate?
                                  (if (> (`self.currentEndDistance`) _array_element_2)
                                    ;;[0.1604 0.5721 1] Set Gate Starting Parameters
                                    (bind _output_get_4 (set `self.gateCurrentDistance` _array_element_2))
                                    (set `self.gateStartDistance` _output_get_4)
                                    (set `self.setGateEnds` true)
                                    ;;[0.1604 0.5721 1] Remove Entry from Array
                                    (`KismetArrayLibrary.Array_Remove` _testdistances _array_index)
                                    (set `self.hasGates` (`KismetArrayLibrary.Array_IsValidIndex` _testdistances))
                                    (break)))))))
                        (:`then_1`
                          (if (`self.setGateEnds`)
                            ;[0.1604 0.5721 1] Set Gate Start
                            (set `self.currentEndDistance` _gatecurrentdistance)
                            (set `self.gateStartLocation` (`SplineComponent.GetLocationAtDistanceAlongSpline` (`self.Spline`) _gatecurrentdistance "Local"))
                            (set `self.gateTestAmount` (`KismetMathLibrary.FTrunc` (/ (- (`SplineComponent.GetSplineLength` (`self.Spline`)) (`self.gateCurrentDistance`)) (`self.gateTestDistance`))))
                            (`|ExecutionSequence`
                              (:`then_0`
                                ;[1 1 1] Find Gate Location
                                ;;[0.1604 0.5721 1] Set Loop Counter/Run Loop
                                (for _ (range (+ (`self.gateTestAmount`) 1))
                                  (`|ExecutionSequence`
                                    (:`then_0`
                                      ;;[0.1604 0.5721 1] First Run Set Gate End Minimum
                                      (`/Engine/EditorBlueprintResources/StandardMacros.DoOnce` false :!label _label_3
                                        (:`Completed`
                                          (bind _output_get_5 (set `self.gateCurrentDistance` (+ (`self.gateCurrentDistance`) (`self.gateSize`))))
                                          (set `self.gateEndDistance` _output_get_5))))
                                    (:`then_1`
                                      ;;[0.1604 0.5721 1] Find Gate End Location/Distance
                                      ;;;[1 1 1] Increment Test Distance
                                      (bind _output_get_6 (set `self.gateCurrentDistance` (+ (`self.gateCurrentDistance`) (`self.gateTestDistance`))))
                                      (bind _returnvalue_12 (`SplineComponent.GetLocationAtDistanceAlongSpline` (`self.Spline`) _output_get_6 "Local"))
                                      ;;;[1 1 1] Test Start-End Length
                                      (if (> (`KismetMathLibrary.Vector_Distance` _returnvalue_12 (`self.gateStartLocation`)) (`self.gateSize`))
                                        ;;;[1 1 1] Set Gate End
                                        (set `self.gateEndLocation` _returnvalue_12)
                                        (set `self.gateEndDistance` (`self.gateCurrentDistance`))
                                        (break))))))
                              (:`then_1`
                                (goto _label_3 :!via `Reset`))
                              (:`then_2`
                                ;;[1 0.7602 0.2323] Add Gate Bounds to Clear
                                (`KismetArrayLibrary.Array_Add` (`self.gateOccupiedArea`) (`KismetMathLibrary.MakeVector2D` (`self.gateStartDistance`) (`self.gateEndDistance`)))
                                (if (`self.hasGates`)
                                  ;;[1 0.7602 0.2323] Clear overlapping Gates
                                  (for (_array_element_3 _array_index_2) _testdistances_3
                                    (for _array_element_4 (`self.gateOccupiedArea`)
                                      (if (`KismetMathLibrary.InRange_FloatFloat` _array_element_3 (`KismetMathLibrary.BreakVector2D` _array_element_4) (`.Y` (`KismetMathLibrary.BreakVector2D` _array_element_4)))
                                        (`KismetArrayLibrary.Array_Remove` _testdistances_3 _array_index_2)
                                        (break)))))
                                ;[1 1 1] Add Gate Mesh
                                (if (not (`self.gapOnly?`))
                                  (bind _returnvalue_13 (`AddComponent|NODE_AddStaticMeshComponent-10` :`RelativeTransform` (`KismetMathLibrary.MakeTransform` (0.0 0.0 0.0) (struct) (`self.gateScale`))))
                                  (`StaticMeshComponent.SetStaticMesh` _returnvalue_13 (`self.gateMesh`))
                                  (`SceneComponent.K2_SetRelativeLocationAndRotation` _returnvalue_13 _gatestartlocation (`KismetMathLibrary.MakeRotator` (.roll (`KismetMathLibrary.FindLookAtRotation` _gatestartlocation (`self.gateEndLocation`))) (.pitch (`KismetMathLibrary.FindLookAtRotation` _gatestartlocation (`self.gateEndLocation`))) (+ (.yaw (`KismetMathLibrary.FindLookAtRotation` _gatestartlocation (`self.gateEndLocation`))) (`KismetMathLibrary.SelectFloat` (`|GetArrayItem` _gaterotations _returnvalue_2) 0.0 (`KismetArrayLibrary.Array_IsValidIndex` _gaterotations _returnvalue_2)))) false false))))))
                        (:`then_2`
                          ;[1 1 1] Add Cap per Section
                          (if (== (`self.capType`) 2)
                            (`self.addCap` (`self.currentStartDistance`))
                            ;[1 1 1] Add Cap to Gate Start (allSections only)
                            (if (`self.setGateEnds`)
                              (`self.addCap` (`self.currentEndDistance`)))
                            (else
                              ;[1 1 1] Add Gaps to Gate (if Override Enabled)
                              (if (and (`self.gate/GapAlwaysCapped?`) (`self.setGateEnds`))
                                (`self.addCap` (`self.gateStartDistance`))
                                (`self.addCap` (`self.gateEndDistance`))))))
                        (:`then_3`
                          ;[1 1 1] Create Fence Section
                          (bind _returnvalue_14 (`AddComponent|NODE_AddSplineMeshComponent-0`))
                          (`SplineMeshComponent.SetStartScale` _returnvalue_14 (`KismetMathLibrary.MakeVector2D` _fencescale_y _fencescale_z) true)
                          (`SplineMeshComponent.SetEndScale` _returnvalue_14 (`KismetMathLibrary.MakeVector2D` _fencescale_y _fencescale_z) true)
                          (`StaticMeshComponent.SetStaticMesh` _returnvalue_14 (`self.fenceMesh`))
                          ;[1 1 1] Set Section Start/End points
                          (`SplineMeshComponent.SetStartAndEnd` _returnvalue_14 (`SplineComponent.GetLocationAtDistanceAlongSpline` _spline _currentstartdistance "Local") _returnvalue_7 (`SplineComponent.GetLocationAtDistanceAlongSpline` _spline _currentenddistance "Local") (`KismetMathLibrary.SelectVector` _returnvalue_7 (`KismetMathLibrary.ClampVectorSize` (`SplineComponent.GetTangentAtDistanceAlongSpline` _spline _currentenddistance "Local") _sectionlength _sectionlength) (and (== (`self.sectionCurrentIndex`) (`self.sectionEndIndex`)) (`self.linearCorners`))) true))))
                    (else
                      (set `self.currentStartDistance` (`KismetMathLibrary.SelectFloat` (+ _startdistance_2 _returnvalue_6) _returnvalue_6 (`self.independentSegments?`)))
                      (goto _label_2))))))
            (else
              (goto _label))))
        (else
          (goto _label))))
    (:`then_1`
      ;[1 1 1] Add Cap per Segment (non Independent)
      (if (and (not (`self.independentSegments?`)) (== (`self.capType`) 3))
        (for _index_3 (range (`SplineComponent.GetNumberOfSplinePoints` _spline_4))
          (`|ExecutionSequence`
            (:`then_0`
              ;[1 0.7602 0.2323] Is Cap Blocked by Gate?
              (for _array_element_5 (`self.gateOccupiedArea`)
                (bind _returnvalue_15 (`SplineComponent.GetDistanceAlongSplineAtSplinePoint` _spline_4 _index_3))
                (if (`KismetMathLibrary.InRange_FloatFloat` _returnvalue_15 (`KismetMathLibrary.BreakVector2D` _array_element_5) (`.Y` (`KismetMathLibrary.BreakVector2D` _array_element_5)))
                  (set `self.capBlocked` true)
                  (break))))
            (:`then_1`
              (if (`self.capBlocked`)
                (set `self.capBlocked` false)
                (else
                  (`self.addCap` _returnvalue_15))))))))
    (:`then_2`
      ;[1 1 1] Add Start/End Caps
      (if (and (not (`self.closeLoop`)) (> _captype 0))
        ;;[0.1604 0.5721 1] Add Cap at Start of Spline (Start/End only)
        (if (== _captype 1)
          (`self.addCap` (`SplineComponent.GetDistanceAlongSplineAtSplinePoint` _spline_5 0))
          ;;[0.1604 0.5721 1] Add Cap at End of Spline
          (`self.addCap` (`SplineComponent.GetDistanceAlongSplineAtSplinePoint` _spline_5 (- (`SplineComponent.GetNumberOfSplinePoints` _spline_5) 1)) :!label _label_4)
          (elif (or (and (== _captype 3) (`self.independentSegments?`)) (== _captype 2))
            (goto _label_4)))))))