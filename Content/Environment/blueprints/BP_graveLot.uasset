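; BP_graveLot lays out a graveyard plot, previewing grave sites and collecting their spawn locations.
; Its construction script sizes lot and margin boxes, then BuildRow steps an optionally staggered grid, tracing down for landscape-tagged ground.
; Overlap boxes and trace hits classify sites as open, obscured or blocked, shown by colored arrows and filtered by spawn flags into SpawnLocations.
; UpdateExistingSpawns prunes invalid spawned-actor references; actual spawning happens outside these graphs.
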(event `self.ReceiveBeginPlay`)

(event `self.ReceiveActorBeginOverlap`
  (params (OtherActor :type "Actor Object Reference")))

(fn `buildRow`
  (params (yLocation :type "Float (double-precision)"))
  (locals (L_currentRowDistance :type "Float (double-precision)") (`L_staggerRow?` :type Boolean :default false) (L_blocked :type Boolean) (L_obscurred :type Boolean) (L_ground :type Boolean) (L_groundLocation :type "Vector Structure" :default (0.0 0.0 0.0)))
  (bind (_returnvalue_x _returnvalue_y) (`KismetMathLibrary.BreakVector` (`self.K2_GetActorLocation`)))
  (bind _lotmargins_x (`KismetMathLibrary.BreakVector2D` (`self.lotMargins`)))
  (bind _lotmargins_x_2 (`KismetMathLibrary.BreakVector2D` (`self.lotMargins`)))
  (bind _l_blocked (`local.L_blocked`))
  (bind _l_obscurred (`local.L_obscurred`))
  (bind (_l_groundlocation_x _l_groundlocation_y) (`KismetMathLibrary.BreakVector` (`local.L_groundLocation`)))
  (bind (_l_groundlocation_x_2 _l_groundlocation_y_2) (`KismetMathLibrary.BreakVector` (`local.L_groundLocation`)))
  (bind _lotend_x (`KismetMathLibrary.BreakVector` (`self.lotEnd`)))
  (bind _returnvalue (not _l_blocked))
  (bind (_returnvalue_x_2 _returnvalue_y_2) (`KismetMathLibrary.BreakVector2D` (/ (`self.graveSize`) (2.0 2.0))))
  (bind _returnvalue_2 (+ _returnvalue_y (`local.yLocation`)))
  (bind _returnvalue_3 (+ (`KismetMathLibrary.SelectFloat` (+ (`self.staggerAmount`) _returnvalue_x) _returnvalue_x (`local.L_staggerRow?`)) (`local.L_currentRowDistance`)))
  ;[1 0.7602 0.2323] sufficient row distance to run loop?
  (if (> (`self.rowDistance`) 50.0)
    ;[0.2778 0.06791 1] should staggerRow?
    (set `local.L_staggerRow?` (== (`KismetMathLibrary.FMod` (`KismetMathLibrary.Conv_IntToDouble` (`self.rowIndex`)) 2.0) 0.0))
    ;[0.2778 0.06791 1] adjust rowDistance for margin
    (set `local.L_currentRowDistance` (+ (`local.L_currentRowDistance`) _lotmargins_x_2))
    ;[1 0.7602 0.2323] run until row distance exceeds lotBounds
    (while (<= (`local.L_currentRowDistance`) (- (`KismetMathLibrary.SelectFloat` (- _lotend_x (`self.staggerAmount`)) _lotend_x (`local.L_staggerRow?`)) _lotmargins_x))
      ;[1 1 1] test graveSite
      (bind (_outhits _returnvalue_4) (`KismetSystemLibrary.LineTraceMultiForObjects` (`KismetMathLibrary.MakeVector` _returnvalue_3 _returnvalue_2 3000.0) (`KismetMathLibrary.MakeVector` _returnvalue_3 _returnvalue_2 -10.0) (`|MakeArray` "ObjectTypeQuery1" :!type "EObjectTypeQuery Enum")))
      ;[1 0.7602 0.2323] found valid hit?
      (if _returnvalue_4
        (`|ExecutionSequence`
          (:`then_0`
            ;[1 1 1] find ground and any obscurring actors at location
            ;;[0.2778 0.06791 1] clear last hitType
            (set `local.L_ground` false)
            (set `local.L_obscurred` false)
            (for _array_element _outhits
              ;;[1 0.7602 0.2323] hit landscapeActor?
              (if (`self.ActorHasTag` (`.HitActor` (`GameplayStatics.BreakHitResult` _array_element)) "landscape")
                ;;[0.2778 0.06791 1] set hit type and location
                (set `local.L_ground` true)
                (set `local.L_groundLocation` (`.Location` (`GameplayStatics.BreakHitResult` _array_element)))
                (else
                  (set `local.L_obscurred` true)))))
          (:`then_1`
            ;[1 0.7602 0.2323] found ground?
            (if (`local.L_ground`)
              ;[1 1 1] build graveSpace
              (bind _returnvalue_5 (`AddComponent|NODE_AddBoxComponent-2`))
              (`BoxComponent.SetBoxExtent` _returnvalue_5 (`KismetMathLibrary.MakeVector` _returnvalue_x_2 _returnvalue_y_2 50.0) true)
              (`SceneComponent.K2_SetWorldLocation` _returnvalue_5 (`KismetMathLibrary.MakeVector` _l_groundlocation_x (+ (* _returnvalue_y_2 0.85) _l_groundlocation_y) 50.0) false false)
              (`|ExecutionSequence`
                (:`then_0`
                  ;[1 1 1] is graveSite blocked by anything?
                  (bind (_outactors _returnvalue_6) (`KismetSystemLibrary.ComponentOverlapActors` _returnvalue_5 (`SceneComponent.K2_GetComponentToWorld` _returnvalue_5) (`|MakeArray` "ObjectTypeQuery1" :!type "EObjectTypeQuery Enum") null (`|MakeArray` self :!type "Actor Object Reference")))
                  ;;[1 0.7602 0.2323] is overlapping anything?
                  (if _returnvalue_6
                    ;;[0.1604 0.5721 1] overlapping any non-landscape actors?
                    (for _array_element_2 _outactors
                      ;;;[1 0.7602 0.2323] is landscape?
                      (if (`self.ActorHasTag` _array_element_2 "landscape")
                        (set `local.L_blocked` false :!label _label)
                        (else
                          (set `local.L_blocked` true)
                          (break))))
                    (else
                      (goto _label))))
                (:`then_1`
                  ;[1 1 1] build headstone marker
                  (bind _returnvalue_7 (`AddComponent|NODE_AddArrowComponent-2` :`RelativeTransform` (`KismetMathLibrary.MakeTransform` (0.0 0.0 100.0) (struct :`Yaw` 90.0))))
                  (`SceneComponent.K2_SetWorldLocation` _returnvalue_7 (`KismetMathLibrary.MakeVector` _l_groundlocation_x_2 _l_groundlocation_y_2 50.0) false false)
                  ;[0.2778 0.06791 1] set arrowColor
                  (`ArrowComponent.SetArrowColor` _returnvalue_7 (`KismetMathLibrary.SelectColor` (struct :`R` 1.0 :`B` 0.031401 :`A` 1.0) (`KismetMathLibrary.SelectColor` (struct :`G` 0.334804 :`B` 1.0 :`A` 1.0) (struct :`G` 1.0 :`B` 0.027592 :`A` 1.0) (`local.L_obscurred`)) (`local.L_blocked`)))
                  ;[1 0.7602 0.2323] add entry to spawnList?
                  (if (or (`self.spawnAll`) (and (`self.spawnOpen`) (not _l_obscurred) _returnvalue) (and (`self.spawnObscurred`) _l_obscurred _returnvalue) (and (`self.spawnBlocked`) _l_blocked))
                    ;[1 1 1] add location to appropriate array
                    (`KismetArrayLibrary.Array_Add` (`self.spawnLocations`) (`local.L_groundLocation`)))
                  ;[0.2778 0.06791 1] increment rowDistance
                  (set `local.L_currentRowDistance` (+ (`local.L_currentRowDistance`) (`self.rowDistance`)) :!label _label_2)))
              (else
                (goto _label_2)))))
        (else
          (goto _label_2))))))

(fn `updateExistingSpawns`
  (bind _spawnedactorlist (`self.spawnedActorList`))
  ;[1 1 1] is spawned actors list filled?
  (if (> (`KismetArrayLibrary.Array_Length` _spawnedactorlist) 0)
    (bind (_arrayindex _arrayelement) (`/Engine/EditorBlueprintResources/StandardMacros.ReverseForEachLoop` _spawnedactorlist)
      (:`LoopBody`
        ;[1 1 1] soft ref valid?
        (if (`KismetSystemLibrary.IsValidSoftObjectReference` _arrayelement)
          (bind _output (`|ConvertAsset` _arrayelement))
          ;[1 1 1] actor valid?
          (if (`KismetSystemLibrary.IsValid` _output)
            ;[1 1 1] actor NOT being destroyed?
            (if (not (not (`self.IsActorBeingDestroyed` _output)))
              ;[1 1 1] remove entry from array if invalid
              (`KismetArrayLibrary.Array_Remove` _spawnedactorlist _arrayindex :!label _label))
            (else
              (goto _label)))
          (else
            (goto _label)))))))

(fn `UserConstructionScript`
  (locals (L_currentColumnDist :type "Float (double-precision)"))
  (bind (_lotend_x _lotend_y) (`KismetMathLibrary.BreakVector` (`self.lotEnd`)))
  (bind _lotbounds (`self.lotBounds`))
  (bind (_lotend_x_2 _lotend_y_2) (`KismetMathLibrary.BreakVector` (`self.lotEnd`)))
  (bind (_lotmargins_x _lotmargins_y) (`KismetMathLibrary.BreakVector2D` (`self.lotMargins`)))
  (bind _lotmargins (`self.lotMargins`))
  (bind (_lotmargins_x_2 _lotmargins_y_2) (`KismetMathLibrary.BreakVector2D` (`self.lotMargins`)))
  (bind (_lotend_x_3 _lotend_y_3) (`KismetMathLibrary.BreakVector` (`self.lotEnd`)))
  (bind (_lotmargins_x_3 _lotmargins_y_3) (`KismetMathLibrary.BreakVector2D` (`self.lotMargins`)))
  (bind (_x _y) (`KismetMathLibrary.BreakVector2D` _lotmargins))
  (bind _returnvalue (/ _lotend_y_2 2.0))
  (bind (_returnvalue_x _returnvalue_y) (`KismetMathLibrary.BreakVector2D` (* _lotmargins (2.0 2.0))))
  (bind _returnvalue_2 (/ _lotend_x_2 2.0))
  (bind _returnvalue_3 (/ (- _lotend_x _returnvalue_x) 2.0))
  (bind _returnvalue_4 (/ (- _lotend_y _returnvalue_y) 2.0))
  ;[1 0.7602 0.2323] prevent lotCreation if ==0
  (if (and (!= _lotend_x_2 0.0) (!= _lotend_y_2 0.0))
    ;[1 1 1] set lot location and bounds
    (`SceneComponent.K2_SetRelativeLocation` _lotbounds (`KismetMathLibrary.MakeVector` _returnvalue_2 _returnvalue) false false)
    (`BoxComponent.SetBoxExtent` _lotbounds (`KismetMathLibrary.MakeVector` _returnvalue_2 _returnvalue 100.0) false)
    ;[1 1 1] create marginBox
    ;;[1 0.7602 0.2323] are margins active?
    (if (or (> _lotmargins_x 0.0) (> _lotmargins_y 0.0))
      (bind _returnvalue_5 (`AddComponent|NODE_AddBoxComponent-1` :`RelativeTransform` (`KismetMathLibrary.MakeTransform` (`KismetMathLibrary.MakeVector` (+ _returnvalue_3 _x) (+ _returnvalue_4 _y)))))
      (`BoxComponent.SetBoxExtent` _returnvalue_5 (`KismetMathLibrary.MakeVector` _returnvalue_3 _returnvalue_4 80.0) false))
    ;[1 1 1] construct grid
    ;;[1 0.7602 0.2323] sufficient column distance to loop
    (if (> (`self.columnDistance`) 100.0)
      ;;[0.2778 0.06791 1] adjsut columnDistance for margin
      (set `local.L_currentColumnDist` (+ (`local.L_currentColumnDist`) _lotmargins_y_2))
      ;;[1 0.7602 0.2323] loop while currentColumnDist is within bounds
      (while (<= (`local.L_currentColumnDist`) (- _lotend_y_3 _lotmargins_y_3))
        ;;[0.1604 0.5721 1] buildRow at location
        (`self.buildRow` (`local.L_currentColumnDist`))
        ;;[0.2778 0.06791 1] increment column distance
        (set `local.L_currentColumnDist` (+ (`local.L_currentColumnDist`) (`self.columnDistance`)))
        ;;[0.2778 0.06791 1] increment rowIndex
        (`/Engine/EditorBlueprintResources/StandardMacros.IncrementInt` (`self.rowIndex`))))))