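; BP_maus is a configurable modular environment building, likely a mausoleum, assembled entirely in the Construction Script.
; Variables swap roof and door meshes, then add handles, with a mirrored second handle and moved lock for double doors.
; Optional columns and crown spawn as static mesh components with adjustable offsets.
; Windows and decor come from mesh arrays paired by index with transform arrays, falling back when a transform is missing.
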(fn `UserConstructionScript`
  (bind (_columnoffset_x _columnoffset_y) (`KismetMathLibrary.BreakVector2D` (`self.columnOffset`)))
  (bind (_columnoffset_x_2 _columnoffset_y_2) (`KismetMathLibrary.BreakVector2D` (`self.columnOffset`)))
  (bind (_crownoffset_x _crownoffset_y) (`KismetMathLibrary.BreakVector2D` (`self.crownOffset`)))
  (bind _decortransform (`self.decorTransform`))
  (bind _windowmesh (`self.windowMesh`))
  (bind _decormesh (`self.decorMesh`))
  (bind _windowtransforms (`self.windowTransforms`))
  (bind _returnvalue (== 0 (`self.doorType`)))
  (`|ExecutionSequence`
    (:`then_0`
      ;[1 1 1] change roof type
      (`StaticMeshComponent.SetStaticMesh` (`self.roof`) (select `bool` (`self.useFlatRoof?`) :`false` "/Game/Environment/meshes/mausoleum/SM_maus_roofAngle.SM_maus_roofAngle" :`true` "/Game/Environment/meshes/mausoleum/SM_maus_roofFlat.SM_maus_roofFlat" :!type "StaticMesh Object Reference")))
    (:`then_1`
      ;[1 1 1] change doorType
      (`StaticMeshComponent.SetStaticMesh` (`self.door`) (select `int` (`self.doorType`) :`0` "/Game/Environment/meshes/mausoleum/SM_maus_door_01.SM_maus_door_01" :`1` "/Game/Environment/meshes/mausoleum/SM_maus_door_02.SM_maus_door_02" :`2` "/Game/Environment/meshes/mausoleum/SM_maus_door_03.SM_maus_door_03" :!type "StaticMesh Object Reference")))
    (:`then_2`
      ;[1 1 1] build doorHandle(s)
      ;;[0.1604 0.5721 1] build baseHandle
      ;;;[1 1 1] position baseHandle
      (bind _returnvalue_2 (`AddComponent|NODE_AddStaticMeshComponent-2` :`RelativeTransform` (`KismetMathLibrary.MakeTransform` (`KismetMathLibrary.MakeVector` (`KismetMathLibrary.SelectFloat` 5.0 -53.0 _returnvalue) 128.0 85.0))))
      ;;;[1 1 1] change handleMesh
      (`StaticMeshComponent.SetStaticMesh` _returnvalue_2 (select `bool` (`self.useFancyHandle?`) :`false` "/Game/Environment/meshes/mausoleum/SM_maus_doorHandle_01.SM_maus_doorHandle_01" :`true` "/Game/Environment/meshes/mausoleum/SM_maus_doorHandle_02.SM_maus_doorHandle_02" :!type "StaticMesh Object Reference"))
      ;;[1 0.7602 0.2323] is doubleDoor?
      (if _returnvalue
        ;;[0.1604 0.5721 1] add secondHandle
        (bind _returnvalue_3 (`AddComponent|NODE_AddStaticMeshComponent-3` :`RelativeTransform` (`KismetMathLibrary.MakeTransform` (-5.0 128.0 85.0) (struct) (-1.0 1.0 1.0))))
        (`StaticMeshComponent.SetStaticMesh` _returnvalue_3 (select `bool` (`self.useFancyHandle?`) :`false` "/Game/Environment/meshes/mausoleum/SM_maus_doorHandle_01.SM_maus_doorHandle_01" :`true` "/Game/Environment/meshes/mausoleum/SM_maus_doorHandle_02.SM_maus_doorHandle_02" :!type "StaticMesh Object Reference"))
        ;;[0.1604 0.5721 1] adjust lock to doubleDoor
        (`SceneComponent.K2_SetRelativeLocation` (`self.lock`) (-5.0 128.0 100.0) false false)))
    (:`then_3`
      ;[1 1 1] build columns
      ;;[1 0.7602 0.2323] are columns enabled?
      (if (> (`self.columnType`) 0)
        ;;[0.1604 0.5721 1] build 1st column
        ;;;[1 1 1] set column location
        (bind _returnvalue_4 (`AddComponent|NODE_AddStaticMeshComponent-4` :`RelativeTransform` (`KismetMathLibrary.MakeTransform` (`KismetMathLibrary.MakeVector` (+ _columnoffset_x_2 94.0) (+ _columnoffset_y_2 159.0)))))
        ;;;[1 1 1] set column meshType
        (`StaticMeshComponent.SetStaticMesh` _returnvalue_4 (select `bool` (== (`self.columnType`) 2) :`false` "/Game/Environment/meshes/mausoleum/SM_maus_col_01.SM_maus_col_01" :`true` "/Game/Environment/meshes/mausoleum/SM_maus_col_02.SM_maus_col_02" :!type "StaticMesh Object Reference"))
        ;;[0.1604 0.5721 1] build 2nd column
        ;;;[1 1 1] set column location
        (bind _returnvalue_5 (`AddComponent|NODE_AddStaticMeshComponent-5` :`RelativeTransform` (`KismetMathLibrary.MakeTransform` (`KismetMathLibrary.MakeVector` (- -94.0 _columnoffset_x) (+ _columnoffset_y 159.0)))))
        ;;;[1 1 1] set column meshType
        (`StaticMeshComponent.SetStaticMesh` _returnvalue_5 (select `bool` (== (`self.columnType`) 2) :`false` "/Game/Environment/meshes/mausoleum/SM_maus_col_01.SM_maus_col_01" :`true` "/Game/Environment/meshes/mausoleum/SM_maus_col_02.SM_maus_col_02" :!type "StaticMesh Object Reference"))))
    (:`then_4`
      ;[1 1 1] build crown
      ;;[1 0.7602 0.2323] is crown enabled?
      (if (> (`self.crownType`) 0)
        ;;[0.1604 0.5721 1] set location/scale
        (bind _returnvalue_6 (`AddComponent|NODE_AddStaticMeshComponent-6` :`RelativeTransform` (`KismetMathLibrary.MakeTransform` (`KismetMathLibrary.MakeVector` 0.0 (+ _crownoffset_x 165.0) (+ _crownoffset_y 290.0)) (struct) (`self.crownScale`))))
        ;;[0.1604 0.5721 1] change mesh type
        (`StaticMeshComponent.SetStaticMesh` _returnvalue_6 (select `int` (- (`self.crownType`) 1) :`0` "/Game/Environment/meshes/mausoleum/SM_maus_cap_01.SM_maus_cap_01" :`1` "/Game/Environment/meshes/mausoleum/SM_maus_cap_02.SM_maus_cap_02" :`2` "/Game/Environment/meshes/mausoleum/SM_maus_cap_03.SM_maus_cap_03" :!type "StaticMesh Object Reference"))))
    (:`then_5`
      ;[1 1 1] build windows
      ;;[1 0.7602 0.2323] are windows enabled?
      (if (`KismetArrayLibrary.Array_IsValidIndex` _windowmesh)
        (for (_ _array_index) _windowmesh
          ;;[0.1604 0.5721 1] add single window
          ;;;[1 1 1] set mesh transform
          (bind _returnvalue_7 (`AddComponent|NODE_AddStaticMeshComponent-7` :`RelativeTransform` (`KismetMathLibrary.SelectTransform` (`|GetArrayItem` _windowtransforms _array_index) (`KismetMathLibrary.MakeTransform` (0.0 0.0 0.0)) (`KismetArrayLibrary.Array_IsValidIndex` _windowtransforms _array_index))))
          ;;;[1 1 1] set mesh type
          (`StaticMeshComponent.SetStaticMesh` _returnvalue_7 (`|GetArrayItem` (`self.windowMesh`) _array_index)))))
    (:`then_6`
      ;[1 1 1] build decor
      ;;[1 0.7602 0.2323] is decor enabled?
      (if (`KismetArrayLibrary.Array_IsValidIndex` _decormesh)
        (for (_ _array_index_2) _decormesh
          ;;[0.1604 0.5721 1] add single decor piece
          ;;;[1 1 1] set mesh transform
          (bind _returnvalue_8 (`AddComponent|NODE_AddStaticMeshComponent-8` :`RelativeTransform` (`KismetMathLibrary.SelectTransform` (`|GetArrayItem` _decortransform _array_index_2) (`KismetMathLibrary.MakeTransform` (0.0 0.0 0.0)) (`KismetArrayLibrary.Array_IsValidIndex` _decortransform _array_index_2))))
          ;;;[1 1 1] set mesh type
          (`StaticMeshComponent.SetStaticMesh` _returnvalue_8 (`|GetArrayItem` (`self.decorMesh`) _array_index_2)))))))